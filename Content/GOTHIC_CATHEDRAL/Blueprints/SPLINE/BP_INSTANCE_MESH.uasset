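; BP_INSTANCE_MESH is a construction-time tool that fills a 3D grid with copies of a chosen static mesh.
; The construction script assigns the mesh to a hierarchical instanced static mesh component and clamps each axis count to at least one.
; Nested Z, Y and X loops add one unrotated, unscaled instance per cell, offset by per-axis spacing.
; The event graph holds no runtime logic.
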(fn `UserConstructionScript`
  (`StaticMeshComponent.SetStaticMesh` (`self.HierarchicalInstancedStaticMesh`) (`self.Mesh`))
  (if (<= (`self.X Number`) 0)
    (set `self.X Number` 1))
  (if (<= (`self.Y Number`) 0)
    (set `self.Y Number` 1))
  (if (<= (`self.Z Number`) 0)
    (set `self.Z Number` 1))
  (for _index (range (`self.Z Number`))
    (for _index_2 (range (`self.Y Number`))
      (for _index_3 (range (`self.X Number`))
        ;[1 1 1] X
        (`InstancedStaticMeshComponent.AddInstance` (`self.HierarchicalInstancedStaticMesh`) (`KismetMathLibrary.MakeTransform` (`KismetMathLibrary.MakeVector` (* _index_3 (`self.X Distance`)) (* _index_2 (`self.Y Distance`)) (* _index (`self.Z Distance`)))))))))