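; Spline construction-script tool that builds a three-part mesh run (start, repeating body, end) with collision along a spline.
; It measures each mesh's bounds along the chosen forward axis, then places the start mesh behind the local origin on X.
; Body segments repeat by mesh length, with clamped tangents limiting stretching.
; The end mesh extends past the spline's end along its tangent, but is spawned inside the body loop, once per iteration.
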(event `self.ReceiveBeginPlay`)

(fn `UserConstructionScript`
  (bind _spline (`self.Spline`))
  (bind _spline_2 (`self.Spline`))
  (bind _mesh_length__auto_detect_ (`self.Mesh_length (auto detect)`))
  (bind _spline_3 (`self.Spline`))
  (bind _returnvalue (`SplineComponent.GetSplineLength` _spline_3))
  (bind (_min _max) (break `Box` (`StaticMesh.GetBoundingBox` (`self.End mesh`))))
  (bind (_min_2 _max_2) (break `Box` (`StaticMesh.GetBoundingBox` (`self.Body mesh`))))
  (bind (_min_3 _max_3) (break `Box` (`StaticMesh.GetBoundingBox` (`self.Start mesh`))))
  (bind _returnvalue_2 (`SplineComponent.GetLocationAtDistanceAlongSpline` _spline_3 _returnvalue "Local"))
  (bind _returnvalue_3 (`KismetMathLibrary.Conv_RotatorToVector` (`SplineComponent.GetRotationAtDistanceAlongSpline` _spline_3 _returnvalue "Local")))
  ;[0.151 0.05585 0.05585] Prepare
  ;;[0.01042 0.01042 0.01042] What Axis you use?
  (if (`|EnumEquality` (`self.Forward Axis`) "X")
    (set `self.Mesh_length (auto detect)` (.x (- _max_2 _min_2)))
    (set `self.Offset_of_start_mesh_` (.x (- _max_3 _min_3)))
    (set `self.End_mesh_length` (.x (- _max _min)))
    (elif (`|EnumEquality` (`self.Forward Axis`) "Y")
      (set `self.Mesh_length (auto detect)` (.y (- _max_2 _min_2)))
      (set `self.Offset_of_start_mesh_` (.y (- _max_3 _min_3)))
      (set `self.End_mesh_length` (.y (- _max _min)))
      (else
        (set `self.Mesh_length (auto detect)` (.z (- _max_2 _min_2)))
        (set `self.Offset_of_start_mesh_` (.z (- _max_3 _min_3)))
        (set `self.End_mesh_length` (.z (- _max _min))))))
  ;[0.1302 0.0448 0.1264] Spawn Start Mesh
  (bind _returnvalue_4 (`AddComponent|NODE_AddSplineMeshComponent-2`))
  (`StaticMeshComponent.SetStaticMesh` _returnvalue_4 (`self.Start mesh`))
  (`SplineMeshComponent.SetForwardAxis` _returnvalue_4 (`self.Forward axis`) true)
  (`SplineMeshComponent.SetStartPosition` _returnvalue_4 (`KismetMathLibrary.MakeVector` (* -1 (`self.Offset_of_start_mesh_`))) true) ; To offset the "start mesh"
  (`SplineMeshComponent.SetEndPosition` _returnvalue_4 (0.0 0.0 0.0) true) ; So the mesh will not exagerate the start point of spline
  (`PrimitiveComponent.SetCollisionEnabled` _returnvalue_4 "QueryAndPhysics")
  ;[0.05174 0.05465 0.07187] Spawn BODY
  (for _index (range (+ (`KismetMathLibrary.FTrunc` (/ (`SplineComponent.GetSplineLength` (`self.Spline`)) (`self.Mesh_length (auto detect)`))) 1))
    (bind _returnvalue_5 (`AddComponent|NODE_AddSplineMeshComponent-1`))
    (`StaticMeshComponent.SetStaticMesh` _returnvalue_5 (`self.Body mesh`))
    (`SplineMeshComponent.SetForwardAxis` _returnvalue_5 (`self.Forward axis`) true)
    (`PrimitiveComponent.SetCollisionEnabled` _returnvalue_5 "QueryAndPhysics")
    (bind _returnvalue_6 (* _index (`self.Mesh_length (auto detect)`)))
    (bind _returnvalue_7 (* (+ _index 1) (`self.Mesh_length (auto detect)`)))
    (`SplineMeshComponent.SetStartAndEnd` _returnvalue_5 (`SplineComponent.GetLocationAtDistanceAlongSpline` _spline_2 _returnvalue_6 "Local") (`KismetMathLibrary.ClampVectorSize` (`SplineComponent.GetTangentAtDistanceAlongSpline` _spline_2 _returnvalue_6 "Local") 0.0 _mesh_length__auto_detect_) (`SplineComponent.GetLocationAtDistanceAlongSpline` _spline _returnvalue_7 "Local") (`KismetMathLibrary.ClampVectorSize` (`SplineComponent.GetTangentAtDistanceAlongSpline` _spline _returnvalue_7 "Local") 0.0 _mesh_length__auto_detect_) true)
    (`SplineMeshComponent.SetStartAndEnd` _returnvalue_5 (`SplineComponent.GetLocationAtDistanceAlongSpline` _spline_2 _returnvalue_6 "Local") (`KismetMathLibrary.ClampVectorSize` (`SplineComponent.GetTangentAtDistanceAlongSpline` _spline_2 _returnvalue_6 "Local") 0.0 _mesh_length__auto_detect_) (`SplineComponent.GetLocationAtDistanceAlongSpline` _spline _returnvalue_7 "Local") (`KismetMathLibrary.ClampVectorSize` (`SplineComponent.GetTangentAtDistanceAlongSpline` _spline _returnvalue_7 "Local") 0.0 _mesh_length__auto_detect_) true)
    ;[0.1042 0.09404 0.02841] Spawn End Mesh
    (bind _returnvalue_8 (`AddComponent|NODE_AddSplineMeshComponent-3`))
    (`StaticMeshComponent.SetStaticMesh` _returnvalue_8 (`self.End mesh`))
    (`SplineMeshComponent.SetForwardAxis` _returnvalue_8 (`self.Forward axis`) true)
    (`SplineMeshComponent.SetStartPosition` _returnvalue_8 _returnvalue_2 true) ; To offset the "start mesh"
    (`SplineMeshComponent.SetEndPosition` _returnvalue_8 (+ _returnvalue_2 (* (`KismetMathLibrary.Normal` (`SplineComponent.GetTangentAtDistanceAlongSpline` _spline_3 _returnvalue "Local")) (`self.End_mesh_length`))) true) ; So the mesh will not exagerate the start point of spline
    (`SplineMeshComponent.SetStartTangent` _returnvalue_8 _returnvalue_3 true)
    (`SplineMeshComponent.SetEndTangent` _returnvalue_8 _returnvalue_3 true)
    (`PrimitiveComponent.SetCollisionEnabled` _returnvalue_8 "QueryAndPhysics")))