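; Actor component that runs branching dialogues with subtitles, voice, body and face montages, and clickable answers.
; StartADialogue runs four tracks, with sound completion advancing montages and untimed subtitles, then showing answers or the next acceptable dialogue.
; A chosen answer replays through the same pipeline as a temporary dialogue, then jumps back by dialogue name.
; Subtitles reach listed players' components, positional sounds multicast, and montages go through BPI_AdvancedDialogue.
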(event `Answer Selected_Event`
  (params (AnswerIndex :type Integer))
  (bind _returnvalue (`GameplayStatics.GetPlayerController` 0))
  (bind (_answertitle _subtitles _sound _dialoguetogo _actor_locationdata) (break `/Game/AdvancedDialogue/Blueprints/Structures/Answer_Structure` (`|GetArrayItem` (`.Answers_29_42967243473DC209CD191088961485B2` (break `/Game/AdvancedDialogue/Blueprints/Structures/AdvancedDialogue_Structure` (`|GetArrayItem` (`self.All Dialogues`) (`self.DialogueIndex`)))) AnswerIndex)))
  ;[1 1 1] On Answer Selected
  (set `self.Came From Answer?` true) ; I used the same codes for answers and normal dialogues. \nI use this boolean to distinguish between the two.
  (bind _output_get (set `self.AnswerDialogue` (`|MakeArray` (make `/Game/AdvancedDialogue/Blueprints/Structures/AdvancedDialogue_Structure` _subtitles _sound _dialoguetogo _actor_locationdata) :!type "/Game/AdvancedDialogue/Blueprints/Structures/AdvancedDialogue_Structure Structure"))) ; Saving the dialogue that should start
  (`self.Reset All Indexes`) ; Resetting all indexes (Dialogue index, Sound index etc)
  (`self.Start A Dialogue` _output_get (`self.Show Subtitles To These Players`)) ; Starting the Answer
  (for _array_element (`self.AnswerWidgets`)
    (`Widget.RemoveFromParent` _array_element))
  (`WidgetBlueprintLibrary.SetInputMode_GameOnly` _returnvalue) ; Setting input mode to Default (You can change these)
  (set `PlayerController.bShowMouseCursor` false _returnvalue))

(event `self.ReceiveBeginPlay`
  ;[1 1 1] Setting the widgets
  ;;[1 1 1] if the owner is locally controlled
  (bind _aspawn (cast `Pawn` (`self.GetOwner`))
    (:`then`
      (if (`Pawn.IsLocallyControlled` _aspawn)
        (bind _returnvalue (`|CreateWidget` "/Game/AdvancedDialogue/Blueprints/Widgets/AdvancedDialogueWidget.AdvancedDialogueWidget_C" (`GameplayStatics.GetPlayerController` 0) :!label _label)) ; Create the widget
        (bind _output_get (set `self.DialogueWidgetRef` _returnvalue)) ; Save the reference of it
        (bind _subtitletext (`/Game/AdvancedDialogue/Blueprints/Widgets/AdvancedDialogueWidget.SubtitleText` _output_get))
        (`TextBlock.SetText` _subtitletext "")
        (bind _output_get_2 (set `self.SubtitleTextRef` _subtitletext)) ; Save the reference of the subtitle text
        (`Widget.SetRenderOpacity` _output_get_2 (`KismetMathLibrary.SelectFloat` 1.0 0.0 (`self.Subtitles On?`)))
        (`ScaleBox.SetUserSpecifiedScale` (`/Game/AdvancedDialogue/Blueprints/Widgets/AdvancedDialogueWidget.ScaleBox_0` _output_get) (`self.SubtitleScale`)) ; Seting Subtitle Scale
        (`UserWidget.AddToPlayerScreen` _output_get 0)
        (for _ (range 9)
          (bind _returnvalue_2 (`|CreateWidget` "/Game/AdvancedDialogue/Blueprints/Widgets/AnAnswer_Widget.AnAnswer_Widget_C"))
          (`ScaleBox.SetUserSpecifiedScale` (`/Game/AdvancedDialogue/Blueprints/Widgets/AnAnswer_Widget.ScaleBox_19` _returnvalue_2) (`self.AnswersScale`)) ; Setting Answer Scale
          (bind _returnvalue_3 (`KismetArrayLibrary.Array_Add` (`self.AnswerWidgets`) _returnvalue_2))
          (set `/Game/AdvancedDialogue/Blueprints/Widgets/AnAnswer_Widget.Answer Index` _returnvalue_3 _returnvalue_2) ; Sending their indexes to Answers Buttons
          (add `/Game/AdvancedDialogue/Blueprints/Widgets/AnAnswer_Widget.Answer Selected` _returnvalue_2 (delegate `Answer Selected_Event`)) ; Binding "AnswerSelected" event dispatchers to an event
        )))
    (:`CastFailed`
      (goto _label))))

(event `Set Subtitle`
  (params (InText :type Text))
  ;[1 1 1] Subtitle
  (bind _subtitletextref (`self.SubtitleTextRef`)
    (:`then`
      (`TextBlock.SetText` _subtitletextref InText))
    (:`else`)))

(event `Next Subtitle`
  (bind _subtitleindex (`self.SubtitleIndex`))
  (bind ((`Subtitles_12_4EBD225F42D27CDC1BAC3EA92E85891E` _subtitles) (`Sound_27_5348D2E84AA695ED1A4D9D8B8F804C14` _sound)) (break `/Game/AdvancedDialogue/Blueprints/Structures/AdvancedDialogue_Structure` (`|GetArrayItem` (`self.All Dialogues`) (`self.DialogueIndex`))))
  (bind (_subtitle _duration) (break `/Game/AdvancedDialogue/Blueprints/Structures/str_Subtitle` (`|GetArrayItem` _subtitles _subtitleindex)))
  ;[1 1 1] Subtitle
  (remove `self.Sound Finished` (delegate `Next Subtitle`))
  (`/Engine/EditorBlueprintResources/StandardMacros.IncrementInt` (`self.SubtitleIndex`) :!label _label_2
    (:`  `
      (`self.TextFinished`)
      (if (`KismetArrayLibrary.Array_IsValidIndex` _subtitles _subtitleindex) :!label _label_3
        (`self.Show Subtitle` _subtitle)
        (bind _subtitletextref (`self.SubtitleTextRef`)
          (:`then`
            (`TextBlock.SetText` _subtitletextref _subtitle)
            (if (!= _duration 0.0)
              (`KismetSystemLibrary.Delay` _duration)
              (goto _label_2)
              (else
                (add `self.Sound Finished` (delegate `Next Subtitle`)))))
          (:`else`))
        (else
          (set `self.SubtitleIndex` 0))))))

(event `Set Subtitles On/Off`
  (params (`Subtitles On?` :type Boolean))
  ;[1 1 1] Subtitle
  (set `self.Subtitles On?` `Subtitles On?`))

(event `Show Subtitle`
  (params (InText :type Text))
  ;[1 1 1] Subtitle
  (for _array_element (`self.Show Subtitles To These Players`)
    (bind _returnvalue (`Actor.GetComponentByClass` _array_element "AdvancedDialogueComponent_C"))
    (`/Engine/EditorBlueprintResources/StandardMacros.IsValid` _returnvalue
      (:`Is Valid`
        (`self.Set Subtitle` _returnvalue InText)))))

(event `Start A Dialogue`
  (params (`Advanced Dialogue` :type "Array of /Game/AdvancedDialogue/Blueprints/Structures/AdvancedDialogue_Structure Structure") (`Show Subtitles to These Players` :type "Array of Actor Object Reference"))
  (bind _soundindex (`self.SoundIndex`))
  (bind ((`Subtitles_12_4EBD225F42D27CDC1BAC3EA92E85891E` _subtitles) (`Sound_27_5348D2E84AA695ED1A4D9D8B8F804C14` _sound)) (break `/Game/AdvancedDialogue/Blueprints/Structures/AdvancedDialogue_Structure` (`|GetArrayItem` (`self.All Dialogues`) (`self.DialogueIndex`))))
  (bind ((`ActortoAffect_17_0778FB784ABBCDF137E55D85C83E3DE5` _actortoaffect) (`Location_9_E4F8D77349A8058105E1AB823D349B55` _location)) (break `/Game/AdvancedDialogue/Blueprints/Structures/str_ActorToAffect` (`.Actor-LocationData_19_8563797E4BC5E97FB11E18AC6DE6991D` (break `/Game/AdvancedDialogue/Blueprints/Structures/AdvancedDialogue_Structure` (`|GetArrayItem` (`self.All Dialogues`) (`self.DialogueIndex`))))))
  (bind (_sound_2 _afterdelay _volume) (break `/Game/AdvancedDialogue/Blueprints/Structures/str_Sound` (`|GetArrayItem` _sound _soundindex)))
  (set `self.All Dialogues` `Advanced Dialogue`) ; Saving the All dialogues (I used the same codes for answers and normal dialogues.\nSo this variable can sometimes contain only the answers)
  ;[1 1 1] Saving the "Show Subtitles to These Players" variable if is valid.
  (if (`KismetArrayLibrary.Array_IsValidIndex` `Show Subtitles to These Players`)
    (`/Engine/EditorBlueprintResources/StandardMacros.IsValid` (`|GetArrayItem` `Show Subtitles to These Players`)
      (:`Is Valid`
        (set `self.Show Subtitles To These Players` `Show Subtitles to These Players`))
      (:`Is Not Valid`
        _)))
  (`|ExecutionSequence`
    (:`then_0`
      (goto _label_3))
    (:`then_1`
      ;[1 1 1] Sound
      (if (`KismetArrayLibrary.Array_IsValidIndex` _sound _soundindex) :!label _label_4
        (if (`KismetSystemLibrary.IsValidSoftObjectReference` _sound_2)
          (bind _returnvalue (`KismetSystemLibrary.LoadAsset_Blocking` _sound_2))
          (`/Engine/EditorBlueprintResources/StandardMacros.IsValid` _actortoaffect
            (:`Is Valid`
              (bind _assound_wave (cast `SoundWave` _returnvalue :!pure true))
              (`self.Spawn Sound Attached` _assound_wave (`Actor.RootComponent` _actortoaffect) _volume)
              (bind _returnvalue_2 (+ (`SoundBase.Duration` _assound_wave) _afterdelay))
              (`KismetSystemLibrary.Delay` _returnvalue_2)
              (`/Engine/EditorBlueprintResources/StandardMacros.IncrementInt` (`self.SoundIndex`) :!label _label_5
                (:`  `
                  _)))
            (:`Is Not Valid`
              (if (== _location (0.0 0.0 0.0) :`ErrorTolerance` 1.0)
                ;;[1 1 1] Not Replicated
                (`GameplayStatics.PlaySound2D` _assound_wave _volume 1.0 0.0 null (`self.GetOwner`))
                (`KismetSystemLibrary.Delay` _returnvalue_2)
                (`/Engine/EditorBlueprintResources/StandardMacros.IncrementInt` (`self.SoundIndex`)
                  (:`  `
                    _))
                (else
                  (`self.Spawn Sound 3D` _assound_wave _volume _location)
                  (`KismetSystemLibrary.Delay` _returnvalue_2)
                  (`/Engine/EditorBlueprintResources/StandardMacros.IncrementInt` (`self.SoundIndex`)
                    (:`  `
                      _))))))
          (else
            (`KismetSystemLibrary.Delay` _afterdelay)
            (goto _label_5)))
        (`self.Sound Finished`)
        (goto _label_4)
        (else
          (set `self.SoundIndex` 0)
          (`self.Start Answers`))))
    (:`then_2`
      (`self.Play Body Montage`))
    (:`then_3`
      (`self.Play Face Montage`))))

(event `Remove Subtitle`
  ;[1 1 1] Subtitle
  (`self.Show Subtitle` ""))

(event `Spawn Sound Attached`
  (params (Sound :type "SoundBase Object Reference") (AttachToComponent :type "SceneComponent Object Reference") (VolumeMultiplier :type "Float (single-precision)"))
  ;[1 1 1] Sound
  (`self.Spawn Sound Attached_Multicast` Sound AttachToComponent VolumeMultiplier))

(event `Spawn Sound Attached_Multicast`
  (params (Sound :type "SoundBase Object Reference") (AttachToComponent :type "SceneComponent Object Reference") (VolumeMultiplier :type "Float (single-precision)"))
  ;[1 1 1] Sound
  (`GameplayStatics.SpawnSoundAttached` Sound AttachToComponent "None" (0.0 0.0 0.0) (struct) "SnapToTarget" false VolumeMultiplier 1.0 0.0 null null))

(event `Spawn Sound 3D_Multicast`
  (params (Sound :type "SoundBase Object Reference") (VolumeMultiplier :type "Float (single-precision)") (Location :type "Vector Structure"))
  ;[1 1 1] Sound
  (`GameplayStatics.SpawnSoundAtLocation` Sound Location (struct) VolumeMultiplier 1.0 0.0 null null))

(event `Spawn Sound 3D`
  (params (Sound :type "SoundBase Object Reference") (VolumeMultiplier :type "Float (single-precision)") (Location :type "Vector Structure"))
  ;[1 1 1] Sound
  (`self.Spawn Sound 3D_Multicast` Sound VolumeMultiplier Location))

(event `Play Body Montage`
  (bind _bodymontageindex (`self.BodyMontageIndex`))
  (bind ((`ActortoAffect_17_0778FB784ABBCDF137E55D85C83E3DE5` _actortoaffect) (`BodyMontage_18_F1DD1D2E406DB4899E2C56B6DBDCC6F3` _bodymontage) (`FaceMontage_19_5A2A02D24D35D2E37F8C3BAF53EA7171` _facemontage)) (break `/Game/AdvancedDialogue/Blueprints/Structures/str_ActorToAffect` (`.Actor-LocationData_19_8563797E4BC5E97FB11E18AC6DE6991D` (break `/Game/AdvancedDialogue/Blueprints/Structures/AdvancedDialogue_Structure` (`|GetArrayItem` (`self.All Dialogues`) (`self.DialogueIndex`))))))
  (bind _animmontage (break `/Game/AdvancedDialogue/Blueprints/Structures/str_AnimMontage` (`|GetArrayItem` _bodymontage _bodymontageindex)))
  ;[1 1 1] Body Anim Montage
  (if (`KismetArrayLibrary.Array_IsValidIndex` _bodymontage _bodymontageindex) :!label _label_6
    (if (`KismetSystemLibrary.IsValidSoftObjectReference` _animmontage)
      (if (`KismetSystemLibrary.DoesImplementInterface` _actortoaffect "/Game/AdvancedDialogue/Blueprints/BPI_AdvancedDialogue.BPI_AdvancedDialogue_C")
        (message `/Game/AdvancedDialogue/Blueprints/BPI_AdvancedDialogue.Play Body Montage` _actortoaffect _animmontage)
        (add `self.Sound Finished` (delegate `Next Body Montage`))
        (else
          (`self.Show Error Message` "ERROR: The Pawn Has Not BPI_AdvancedDialogue interface."))))
    (else
      (set `self.BodyMontageIndex` 0)
      (`self.BodyMontagesFinished`))))

(event `Next Body Montage`
  ;[1 1 1] Body Anim Montage
  (remove `self.Sound Finished` (delegate `Next Body Montage`))
  (`/Engine/EditorBlueprintResources/StandardMacros.IncrementInt` (`self.BodyMontageIndex`)
    (:`  `
      (goto _label_6))))

(event `Play Face Montage`
  (bind _facemontageindex (`self.FaceMontageIndex`))
  (bind ((`ActortoAffect_17_0778FB784ABBCDF137E55D85C83E3DE5` _actortoaffect) (`BodyMontage_18_F1DD1D2E406DB4899E2C56B6DBDCC6F3` _bodymontage) (`FaceMontage_19_5A2A02D24D35D2E37F8C3BAF53EA7171` _facemontage)) (break `/Game/AdvancedDialogue/Blueprints/Structures/str_ActorToAffect` (`.Actor-LocationData_19_8563797E4BC5E97FB11E18AC6DE6991D` (break `/Game/AdvancedDialogue/Blueprints/Structures/AdvancedDialogue_Structure` (`|GetArrayItem` (`self.All Dialogues`) (`self.DialogueIndex`))))))
  (bind _animmontage (break `/Game/AdvancedDialogue/Blueprints/Structures/str_AnimMontage` (`|GetArrayItem` _facemontage _facemontageindex)))
  ;[1 1 1] Face Anim Montage
  (if (`KismetArrayLibrary.Array_IsValidIndex` _facemontage _facemontageindex) :!label _label_7
    (if (`KismetSystemLibrary.IsValidSoftObjectReference` _animmontage)
      (if (`KismetSystemLibrary.DoesImplementInterface` _actortoaffect "/Game/AdvancedDialogue/Blueprints/BPI_AdvancedDialogue.BPI_AdvancedDialogue_C")
        (message `/Game/AdvancedDialogue/Blueprints/BPI_AdvancedDialogue.Play Face Montage` _actortoaffect _animmontage)
        (add `self.Sound Finished` (delegate `Next Face Montge`) :!label _label_8)
        (else
          (`self.Show Error Message` "ERROR: The Pawn Has Not BPI_AdvancedDialogue interface.")))
      (else
        (goto _label_8)))
    (else
      (set `self.FaceMontageIndex` 0)
      (`self.FaceMontagesFinished`))))

(event `Next Face Montge`
  ;[1 1 1] Face Anim Montage
  (remove `self.Sound Finished` (delegate `Next Face Montge`))
  (`/Engine/EditorBlueprintResources/StandardMacros.IncrementInt` (`self.FaceMontageIndex`)
    (:`  `
      (goto _label_7))))

(event `Start Answers`
  (bind _returnvalue (`GameplayStatics.GetPlayerController` 0))
  (bind _all_dialogues (`self.All Dialogues`))
  (bind _dialogueindex (`self.DialogueIndex`))
  (bind _answerwidgets (`self.AnswerWidgets`))
  (bind _all_dialogues_2 (`self.All Dialogues`))
  (bind ((`Answers_29_42967243473DC209CD191088961485B2` _answers)) (break `/Game/AdvancedDialogue/Blueprints/Structures/AdvancedDialogue_Structure` (`|GetArrayItem` _all_dialogues_2 _dialogueindex)))
  ;[1 1 1] Answers
  (bind _aspawn (cast `Pawn` (`self.GetOwner`))
    (:`then`
      (if (`Pawn.IsLocallyControlled` _aspawn)
        (if (`self.Came From Answer?`) :!label _label_9
          (bind (_array_index _success_) (`self.Find Dialogue To Go` (`.DialogueName_16_8B71B0D349F86386E1560CBD6C40D5CD` (break `/Game/AdvancedDialogue/Blueprints/Structures/AdvancedDialogue_Structure` (`|GetArrayItem` (`self.All Dialogues`))))))
          (if _success_
            (set `self.DialogueIndex` _array_index)
            (set `self.Came From Answer?` false)
            (`self.Start A Dialogue` (`self.All Dialogues_GRAND`) (`self.Show Subtitles To These Players`))
            (else
              (`self.Show Error Message` "ERROR: Dialogue to Go value is not same with the Dialogue Names")))
          (elif (`KismetArrayLibrary.Array_IsValidIndex` _answers)
            (set `self.All Dialogues_GRAND` _all_dialogues_2) ; We save it for later use.
            (bind _subtitletextref (`self.SubtitleTextRef`)
              (:`then`
                (`TextBlock.SetText` _subtitletextref ""))
              (:`else`
                _))
            (`self.Remove Subtitle`)
            (set `PlayerController.bShowMouseCursor` true _returnvalue)
            (if (`KismetArrayLibrary.Array_IsValidIndex` _answerwidgets)
              (`WidgetBlueprintLibrary.SetInputMode_GameAndUIEx` _returnvalue (`/Game/AdvancedDialogue/Blueprints/Widgets/AnAnswer_Widget.Button_0` (`|GetArrayItem` _answerwidgets)) "DoNotLock" false)
              (else
                (`WidgetBlueprintLibrary.SetInputMode_GameAndUIEx` _returnvalue null "DoNotLock" false)))
            ;;[1 1 1] We display the answers on the screen.
            (bind _dialoguewidgetref (`self.DialogueWidgetRef`)
              (:`then`
                (for (_array_element _array_index_2) _answers
                  (bind _output (`|GetArrayItem` (`self.AnswerWidgets`) _array_index_2))
                  (`TextBlock.SetText` (`/Game/AdvancedDialogue/Blueprints/Widgets/AnAnswer_Widget.AnswerText` _output) (`.AnswerTitle_32_2406080340DF332B8456939C4E44BCCA` (break `/Game/AdvancedDialogue/Blueprints/Structures/Answer_Structure` _array_element)))
                  (`PanelWidget.AddChild` (`/Game/AdvancedDialogue/Blueprints/Widgets/AdvancedDialogueWidget.VerticalBox_0` _dialoguewidgetref) _output)))
              (:`else`))
            (else
              (bind _result (`/Engine/EditorBlueprintResources/StandardMacros.IncrementInt` _dialogueindex :!label _label_10)
                (:`  `
                  (if (`KismetArrayLibrary.Array_IsValidIndex` _all_dialogues _result)
                    (bind ((`DialogueName_16_8B71B0D349F86386E1560CBD6C40D5CD` _dialoguename) (`Next-Acceptable_31_2D709C4A4FEA672EAC3260B02ABCC796` _next_acceptable)) (break `/Game/AdvancedDialogue/Blueprints/Structures/AdvancedDialogue_Structure` (`|GetArrayItem` _all_dialogues _result)))
                    (`self.Dialogue Finished` _dialoguename)
                    (if _next_acceptable
                      (`self.Start A Dialogue` _all_dialogues (`self.Show Subtitles To These Players`))
                      (else
                        (goto _label_10)))
                    (else
                      ;[1 1 1] dialogue finished
                      (`self.Dialogue Finished` (`.DialogueName_16_8B71B0D349F86386E1560CBD6C40D5CD` (break `/Game/AdvancedDialogue/Blueprints/Structures/AdvancedDialogue_Structure` (`|GetArrayItem` (`self.All Dialogues`) (- (`self.DialogueIndex`) 1)))))
                      (`self.AllDialoguesFinished`)
                      (`TextBlock.SetText` (`self.SubtitleTextRef`) "")
                      (`self.Reset All Indexes`)
                      (`self.Remove Subtitle`))))))))))
    (:`CastFailed`
      (goto _label_9))))

(fn `Find Dialogue To Go`
  (params (`item to find` :type String))
  (returns (`Array Index` :type Integer) (`Success?` :type Boolean))
  (for (_array_element _array_index) (`self.All Dialogues_GRAND`)
    (if (`KismetStringLibrary.EqualEqual_StrStr` (`.DialogueName_16_8B71B0D349F86386E1560CBD6C40D5CD` (break `/Game/AdvancedDialogue/Blueprints/Structures/AdvancedDialogue_Structure` _array_element)) `item to find`)
      (return _array_index true)))
  (return 0 false))

(fn `OnRep_Subtitles On?`
  (bind _subtitletextref (`self.SubtitleTextRef`)
    (:`then`
      (`Widget.SetRenderOpacity` _subtitletextref (`KismetMathLibrary.SelectFloat` 1.0 0.0 (`self.Subtitles On?`))))
    (:`else`
      _))
  (return))

(fn `Reset All Indexes`
  (set `self.DialogueIndex` 0)
  (set `self.SubtitleIndex` 0)
  (set `self.BodyMontageIndex` 0)
  (set `self.FaceMontageIndex` 0)
  (set `self.SoundIndex` 0)
  (return))

(fn `Set Answers Sizes`
  (params (`New Scale` :type "Float (single-precision)" :default 1.0))
  (bind _answerwidgets (`self.AnswerWidgets`))
  (if (`KismetArrayLibrary.Array_IsValidIndex` _answerwidgets)
    (for _array_element _answerwidgets
      (`ScaleBox.SetUserSpecifiedScale` (`/Game/AdvancedDialogue/Blueprints/Widgets/AnAnswer_Widget.ScaleBox_19` _array_element) `New Scale`)))
  (return))

(fn `Set Subtitle Size`
  (params (`New Scale` :type "Float (single-precision)" :default 1.0))
  (bind _dialoguewidgetref (`self.DialogueWidgetRef`)
    (:`then`
      (`ScaleBox.SetUserSpecifiedScale` (`/Game/AdvancedDialogue/Blueprints/Widgets/AdvancedDialogueWidget.ScaleBox_0` _dialoguewidgetref) `New Scale`))
    (:`else`
      _))
  (return))

(fn `Show Error Message`
  (params (InString :type String))
  (`KismetSystemLibrary.PrintString` InString true true (struct :`R` 1.0 :`G` 0.034584 :`A` 1.0) 10.0)
  (`KismetSystemLibrary.PrintString` InString true true (struct :`R` 1.0 :`G` 0.034584 :`A` 1.0) 10.0)
  (`KismetSystemLibrary.PrintString` InString true true (struct :`R` 1.0 :`G` 0.034584 :`A` 1.0) 10.0)
  (return))