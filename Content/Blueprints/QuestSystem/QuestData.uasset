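; QuestData is a quest component that gathers the quests attached to its owning actor.
; On BeginPlay it runs CountQuestActors only when the player character fails the cast to ThirdPersonCharacter; a successful cast does nothing.
; CountQuestActors scans the owner's directly attached actors, adds Quest_Parent instances uniquely to AssociatedQuests, and prints the array length.
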(event `self.ReceiveBeginPlay`
  (cast `/Game/Blueprints/Player/ThirdPersonCharacter` (`GameplayStatics.GetPlayerCharacter` 0)
    (:`CastFailed`
      (`self.CountQuestActors`))))

(event `CountQuestActors`
  (for _array_element (`Actor.GetAttachedActors` (`self.GetOwner`) true false)
    (bind _asquest_parent (cast `/Game/Blueprints/QuestSystem/Quest_Parent` _array_element))
    (`KismetArrayLibrary.Array_AddUnique` (`self.AssociatedQuests`) _asquest_parent))
  (`KismetSystemLibrary.PrintString` (`KismetStringLibrary.Conv_IntToString` (`KismetArrayLibrary.Array_Length` (`self.AssociatedQuests`)))))