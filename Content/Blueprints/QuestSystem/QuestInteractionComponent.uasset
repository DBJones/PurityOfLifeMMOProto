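; Quest interaction component that detects the actor in front of its owner and lets the player interact with quest-bearing targets.
; A per-tick forward sphere trace updates QuestTarget, calls its LookAtMessage and drives the HUD interact prompt.
; The interact input sends the target to a server event, which matches attached Quest_Parent actors against its QuestData quests and currently only prints the resulting name.
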(event `self.ReceiveBeginPlay`
  (if (== (`self.GetOwner`) (`GameplayStatics.GetPlayerCharacter` 0))
    (bind _asmouse_controller (cast `/Game/Blueprints/Mouse_Controller` (`GameplayStatics.GetPlayerController` 0)))
    (bind _output_get (set `self.As Mouse Controller` _asmouse_controller))
    (set `self.W HUD` (`/Game/Blueprints/Mouse_Controller.W_HUD` _output_get))))

(event `self.ReceiveTick`
  (params (DeltaSeconds :type "Float (single-precision)"))
  (`self.InteractionTrace`))

(event `InputAction|Interaction` :overrideparent false
  (params (Key :type "Key Structure"))
  (:`Pressed`
    (bind _questtarget (`self.QuestTarget`)
      (:`then`
        (`self.Server_Interact` _questtarget))
      (:`else`))))

(event `Server_Interact`
  (params (Target :type "Actor Object Reference"))
  (bind _returnvalue (`Actor.GetComponentByClass` Target "/Game/Blueprints/QuestSystem/QuestData.QuestData_C"))
  (bind _associatedquests (`/Game/Blueprints/QuestSystem/QuestData.AssociatedQuests` _returnvalue))
  (cast `/Game/Blueprints/Player/ThirdPersonCharacter` Target
    (:`CastFailed`
      (`/Engine/EditorBlueprintResources/StandardMacros.IsValid` _returnvalue
        (:`Is Valid`
          (bind _w_hud (`self.W HUD`)
            (:`then`
              (`/Game/Blueprints/UI/Interaction/Interact_Item.ToggleVisiblity` (`/Game/Blueprints/UI/HeadsUpDisplay.Interact_Item` _w_hud)))
            (:`else`
              _))
          (for _array_element (`Actor.GetAttachedActors` (`self.QuestTarget`) true false)
            (bind _asquest_parent (cast `/Game/Blueprints/QuestSystem/Quest_Parent` _array_element))
            (if (`KismetArrayLibrary.Array_IsValidIndex` _associatedquests (`KismetArrayLibrary.Array_Find` _associatedquests _asquest_parent))
              (set `self.As Quest Parent` _asquest_parent)))
          (`KismetSystemLibrary.PrintString` (`KismetTextLibrary.Conv_TextToString` (`/Game/Blueprints/QuestSystem/Quest_Parent.Name` (`self.As Quest Parent`)))))))))

(fn `InteractionTrace`
  (bind _returnvalue (`self.GetOwner`))
  (bind _returnvalue_2 (`Actor.K2_GetActorLocation` _returnvalue))
  (bind (_outhit _returnvalue_3) (`KismetSystemLibrary.SphereTraceSingle` _returnvalue_2 (+ _returnvalue_2 (* (`Actor.GetActorForwardVector` _returnvalue) (`self.IntRange`))) 70.0 "TraceTypeQuery4" false (`|MakeArray` _returnvalue) "None" true (struct :`R` 1.0 :`A` 1.0) (struct :`G` 1.0 :`A` 1.0) 2.0))
  (if _returnvalue_3
    (bind (_bblockinghit _binitialoverlap _time _distance _location _impactpoint _normal _impactnormal _physmat _hitactor) (`GameplayStatics.BreakHitResult` _outhit))
    (if (!= (`self.QuestTarget`) _hitactor)
      (bind _output_get (set `self.QuestTarget` _hitactor))
      (message `/Game/Blueprints/Items/Inventory/IInteractInterface.LookAt` _output_get)
      (bind _w_hud (`self.W HUD`)
        (:`then`
          (`Widget.SetVisibility` (`/Game/Blueprints/UI/HeadsUpDisplay.Interact_Item` _w_hud) "Visible"))
        (:`else`)))
    (else
      (set `self.QuestTarget` null)
      (bind _w_hud_2 (`self.W HUD`)
        (:`then`
          (`Widget.SetVisibility` (`/Game/Blueprints/UI/HeadsUpDisplay.Interact_Item` _w_hud_2) "Hidden"))
        (:`else`)))))