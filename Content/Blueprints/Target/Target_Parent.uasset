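; Base Blueprint for targetable enemies, handling click targeting, health, damage and death.
; On BeginPlay it derives HP from level, enemy-type tag and armor, then loads level-based armor and weapon stats from tables, after HP is calculated.
; Ability damage updates health and spawns temporary damage numbers.
; Lethal hits interrupt the caster's casting, clear overlapping abilities and award type-scaled EXP to the player's first active skill.
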(event `self.ReceiveBeginPlay`
  ;[1 1 1] Initialization
  (`|ExecutionSequence`
    (:`then_0`
      (bind _asmouse_controller (cast `/Game/Blueprints/Mouse_Controller` (`GameplayStatics.GetPlayerController` 0)))
      (set `self.As Mouse Controller` _asmouse_controller)
      (`self.DetermineEnemyTypeMultiplier`)
      (bind _outhealth (`self.Calculate HP`))
      (set `self.Current Health` (`KismetMathLibrary.Conv_IntToDouble` _outhealth))
      (set `self.Max Health` (`KismetMathLibrary.Conv_IntToDouble` _outhealth))
      (`self.DetermineWeaponAndArmorStrength`))
    (:`then_1`
      (bind _asname_plate (cast `/Game/Blueprints/Player/NamePlate` (`WidgetComponent.GetWidget` (`self.NamePlate`))))
      (set `/Game/Blueprints/Player/NamePlate.Owner` self _asname_plate))
    (:`then_2`
      (bind _asthird_person_character (cast `/Game/Blueprints/Player/ThirdPersonCharacter` (`GameplayStatics.GetPlayerCharacter` 0)))
      (set `self.PlayerRef` _asthird_person_character))))

(event `self.ReceiveActorOnClicked`
  (params (ButtonPressed :type "Key Structure"))
  (bind _as_mouse_controller (`self.As Mouse Controller`))
  ;[1 1 1] Targetting
  (`/Game/Blueprints/Mouse_Controller.SetTarget` _as_mouse_controller self)
  (add `/Game/Blueprints/Mouse_Controller.TargetChanged` _as_mouse_controller (delegate `ClearTarget`))
  (`SceneComponent.SetVisibility` (`self.TargetIndicator`) true false))

(event `ClearTarget`
  ;[1 1 1] Targetting
  (`SceneComponent.SetVisibility` (`self.TargetIndicator`) false false))

(event `self.ReceiveAnyDamage`
  (params (Damage :type "Float (single-precision)") (DamageType :type "DamageType Object Reference") (InstigatedBy :type "Controller Object Reference") (DamageCauser :type "Actor Object Reference"))
  ;[1 1 1] Damage
  (bind _asability (cast `/Game/Blueprints/Abilities/Ability` DamageCauser))
  (if (>= Damage (`self.Current Health`))
    (bind _asthird_person_character (cast `/Game/Blueprints/Player/ThirdPersonCharacter` (`/Game/Blueprints/Abilities/Ability.Caster` _asability))
      (:`then`
        (`/Game/Blueprints/Player/ThirdPersonCharacter.InterruptCasting` _asthird_person_character))
      (:`CastFailed`
        _))
    (if (`KismetSystemLibrary.IsValid` DamageCauser)
      (`self.K2_DestroyActor` DamageCauser))
    (`self.EnemyDeath`)
    (else
      (bind _output_get (set `self.Current Health` (- (`self.Current Health`) Damage)))
      (set `self.Health_normalized` (`KismetMathLibrary.NormalizeToRange` _output_get 0.0 (`self.Max Health`)))
      (`self.TargetDamaged`)
      (bind _childoutput (`self.UpdateDamageUI` Damage _asability))
      (`KismetSystemLibrary.Delay` 1.2)
      (`Widget.RemoveFromParent` _childoutput))))

(event `EnemyDeath`
  ;[1 1 1] NPC Death
  (set `self.Dead?` true)
  (bind _outexp (`self.CalculateEXPRewardforKO`))
  (`/Game/Blueprints/Skills/Skill_Parent.LevelUpGainExp` (`|GetArrayItem` (`/Game/Blueprints/Player/ThirdPersonCharacter.ActiveSkills` (`self.PlayerRef`))) _outexp)
  (for _array_element (`self.GetOverlappingActors` "/Game/Blueprints/Abilities/Ability.Ability_C")
    (`self.K2_DestroyActor` _array_element))
  (`self.K2_DestroyActor`)
  (`self.TargetKOd`))

(fn `Calculate HP`
  (returns (OutHealth :type Integer))
  (bind _levelmult (`self.Calculate Level Mult`))
  (return (`KismetMathLibrary.FTrunc` (* (/ _levelmult 3.0) (`self.EnemyTypeMultiplier`) (+ (`KismetMathLibrary.Conv_IntToDouble` (`self.Armor Rating`)) 200.0)))))

(fn `Calculate Level Mult`
  (returns (LevelMult :type "Float (double-precision)"))
  (return (`KismetMathLibrary.MultiplyMultiply_FloatFloat` (`KismetMathLibrary.Conv_IntToDouble` (`self.Level`)) 0.85)))

(fn `CalculateEXPRewardforKO`
  (returns (OutEXP :type Integer))
  (if (`BlueprintGameplayTagLibrary.DoesContainerMatchTagQuery` (`self.EnemyType`) (`BlueprintGameplayTagLibrary.MakeGameplayTagQuery` (struct :`TagDictionary` (struct :`(TagName` "EnemyType.RaidBoss")) :`QueryTokenStream` "(0,1,2,1,0)" :`AutoDescription` " ALL( EnemyType.RaidBoss )")))
    _
    (elif (`BlueprintGameplayTagLibrary.DoesContainerMatchTagQuery` (`self.EnemyType`) (`BlueprintGameplayTagLibrary.MakeGameplayTagQuery` (struct :`TagDictionary` (struct :`(TagName` "EnemyType.DungeonBoss")) :`QueryTokenStream` "(0,1,2,1,0)" :`AutoDescription` " ALL( EnemyType.DungeonBoss )")))
      _
      (elif (`BlueprintGameplayTagLibrary.DoesContainerMatchTagQuery` (`self.EnemyType`) (`BlueprintGameplayTagLibrary.MakeGameplayTagQuery` (struct :`TagDictionary` (struct :`(TagName` "EnemyType.High")) :`QueryTokenStream` "(0,1,2,1,0)" :`AutoDescription` " ALL( EnemyType.High )")))
        (return (`KismetMathLibrary.FTrunc` (* (`KismetMathLibrary.MultiplyMultiply_FloatFloat` (- (`KismetMathLibrary.Conv_IntToDouble` (`self.Level`)) 0.5) 0.2) 450.0)))
        (elif (`BlueprintGameplayTagLibrary.DoesContainerMatchTagQuery` (`self.EnemyType`) (`BlueprintGameplayTagLibrary.MakeGameplayTagQuery` (struct :`TagDictionary` (struct :`(TagName` "EnemyType.Mid")) :`QueryTokenStream` "(0,1,2,1,0)" :`AutoDescription` " ALL( EnemyType.Mid )")))
          (return (`KismetMathLibrary.FTrunc` (* (`KismetMathLibrary.MultiplyMultiply_FloatFloat` (- (`KismetMathLibrary.Conv_IntToDouble` (`self.Level`)) 0.5) 0.2) 250.0)))
          (else
            (return (`KismetMathLibrary.FTrunc` (* (`KismetMathLibrary.MultiplyMultiply_FloatFloat` (- (`KismetMathLibrary.Conv_IntToDouble` (`self.Level`)) 0.5) 0.2) 150.0))))))))
  (return (`KismetMathLibrary.FTrunc` (* (`KismetMathLibrary.MultiplyMultiply_FloatFloat` (- (`KismetMathLibrary.Conv_IntToDouble` (`self.Level`)) 0.5) 0.2) 1500.0))))

(fn `DetermineEnemyTypeMultiplier`
  (if (`BlueprintGameplayTagLibrary.DoesContainerMatchTagQuery` (`self.EnemyType`) (`BlueprintGameplayTagLibrary.MakeGameplayTagQuery` (struct :`TagDictionary` (struct :`(TagName` "EnemyType.RaidBoss")) :`QueryTokenStream` "(0,1,2,1,0)" :`AutoDescription` " ALL( EnemyType.RaidBoss )")))
    (set `self.EnemyTypeMultiplier` 50.0)
    (elif (`BlueprintGameplayTagLibrary.DoesContainerMatchTagQuery` (`self.EnemyType`) (`BlueprintGameplayTagLibrary.MakeGameplayTagQuery` (struct :`TagDictionary` (struct :`(TagName` "EnemyType.DungeonBoss")) :`QueryTokenStream` "(0,1,2,1,0)" :`AutoDescription` " ALL( EnemyType.DungeonBoss )")))
      (set `self.EnemyTypeMultiplier` 20.0)
      (elif (`BlueprintGameplayTagLibrary.DoesContainerMatchTagQuery` (`self.EnemyType`) (`BlueprintGameplayTagLibrary.MakeGameplayTagQuery` (struct :`TagDictionary` (struct :`(TagName` "EnemyType.High")) :`QueryTokenStream` "(0,1,2,1,0)" :`AutoDescription` " ALL( EnemyType.High )")))
        (set `self.EnemyTypeMultiplier` 4.0)
        (elif (`BlueprintGameplayTagLibrary.DoesContainerMatchTagQuery` (`self.EnemyType`) (`BlueprintGameplayTagLibrary.MakeGameplayTagQuery` (struct :`TagDictionary` (struct :`(TagName` "EnemyType.Mid")) :`QueryTokenStream` "(0,1,2,1,0)" :`AutoDescription` " ALL( EnemyType.Mid )")))
          (set `self.EnemyTypeMultiplier` 1.67)
          (else
            (set `self.EnemyTypeMultiplier` 0.67)))))))

(fn `DetermineWeaponAndArmorStrength`
  (bind _tableofnpcarmorvalues_defensevalues (break `/Game/Blueprints/Player/LevelledArmorAndWeaponData/LevelledNPCArmorValues` (`self.TableOfNPCArmorValues`)))
  (bind _tableofnpcweaponvalues_defaultweaponstrength (break `/Game/Blueprints/Player/LevelledArmorAndWeaponData/LevelledWeaponStrength` (`self.TableOfNPCWeaponValues`)))
  (bind _returnvalue (* (`BlueprintMapLibrary.Map_Find` _tableofnpcarmorvalues_defensevalues (`self.Level`)) 5))
  (bind _output_get (set `self.Armor Rating` _returnvalue))
  (set `self.Magical Defense` _returnvalue)
  (set `self.Physical Defense` _returnvalue)
  (bind _output_get_2 (set `self.WeaponStrength` (`BlueprintMapLibrary.Map_Find` _tableofnpcweaponvalues_defaultweaponstrength (`self.Level`))))
  (`KismetSystemLibrary.PrintString` (`KismetStringLibrary.Concat_StrStr` "Armor Rating: " (`KismetStringLibrary.Conv_IntToString` _output_get) " Weapon Rating: " (`KismetStringLibrary.Conv_IntToString` _output_get_2)) true true (struct :`G` 0.66 :`B` 1.0 :`A` 1.0) 10.0))

(fn `UpdateDamageUI`
  (params (DamageAmount :type "Float (double-precision)") (DamageCauser :type "/Game/Blueprints/Abilities/Ability Object Reference"))
  (returns (ChildOutput :type "/Game/Blueprints/Target/DamageNumber Object Reference"))
  (bind _ability_details_name (break `/Game/Blueprints/Abilities/AbilityDetails` (`/Game/Blueprints/Abilities/Ability.Ability Details` DamageCauser)))
  (bind _asdamage_number_container (cast `/Game/Blueprints/Target/DamageNumber_Container` (`WidgetComponent.GetWidget` (`self.DamageWidget`))))
  (bind _returnvalue (`|CreateWidget` "/Game/Blueprints/Target/DamageNumber.DamageNumber_C" null _ability_details_name DamageAmount))
  (`StackBox.AddChildToStackBox` (`/Game/Blueprints/Target/DamageNumber_Container.UIContainer` _asdamage_number_container) _returnvalue)
  (return _returnvalue))

(fn `UserConstructionScript`)