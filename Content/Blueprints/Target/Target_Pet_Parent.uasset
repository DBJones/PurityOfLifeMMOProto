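; Base Blueprint for combat pets that belong to an owner character and auto-attack enemies.
; On BeginPlay it passes the owner to its DefaultAI_Pet controller and binds the auto-attack timer setup.
; Starting auto-attack updates combat state, notifies a player owner not yet in combat, and loops spawning attack actors at the controller's EnemyTarget.
; Dismiss plays a sound, makes the pet untargettable and destroys it after a short delay.
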(event `self.ReceiveBeginPlay`
  (`parent.ReceiveBeginPlay`)
  (bind _asdefault_ai_pet (cast `/Game/Blueprints/Target/AI/DefaultAI_Pet` (`AIBlueprintHelperLibrary.GetAIController` self)))
  (set `/Game/Blueprints/Target/AI/DefaultAI_Pet.Pet Owner` (`self.PetOwner`) _asdefault_ai_pet)
  (`/Game/Blueprints/Target/AI/DefaultAI_Pet.SetPlayerOwner` _asdefault_ai_pet)
  (add `self.SetAutoAttackTimer` (`|CreateDelegate` :!event `BeginSetAutoAttackTimer`)))

(event `Kill`
  (`KismetSystemLibrary.Delay` 0.5)
  (`self.K2_DestroyActor`))

(event `BeginSetAutoAttackTimer`
  (bind _petowner (`self.PetOwner`))
  (if (not (`/Game/Blueprints/Character_Base_for_MMO.InCombat?` _petowner))
    (set `self.InCombat?` true)
    (if (== _petowner (`GameplayStatics.GetPlayerCharacter` 0))
      (`self.CharacterDamaged` _petowner)))
  (`self.AutoAttackEvent`)
  (bind _returnvalue (`KismetSystemLibrary.K2_SetTimerDelegate` (delegate `AutoAttackEvent`) 2.5 true))
  (set `self.AutoAttackTimer` _returnvalue))

(event `AutoAttackEvent`
  (bind _asdefault_ai_pet (cast `/Game/Blueprints/Target/AI/DefaultAI_Pet` (`AIBlueprintHelperLibrary.GetAIController` self)))
  (bind _enemytarget (`/Game/Blueprints/Target/AI/DefaultAI_Pet.EnemyTarget` _asdefault_ai_pet)
    (:`then`
      (`|SpawnActorFromClass` (`self.AutoAttack`) (`self.GetTransform` self) "Undefined" "OverrideRootScale" null self _enemytarget null))
    (:`else`)))

(fn `Dismiss`
  (`/Game/Blueprints/Character_Base_for_MMO.PetRef` (`self.PetOwner`)
    (:`then`
      (`GameplayStatics.PlaySoundAtLocation` (`self.DismissCue`) (`self.K2_GetActorLocation` self) (struct) 1.0 1.0 0.0 null null null null)
      (set `self.Targettable?` false)
      (`self.Kill`))
    (:`else`)))

(fn `UserConstructionScript`
  (`parent.UserConstructionScript`))