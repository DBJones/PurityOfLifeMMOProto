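; Test melee enemy character that detects the player and hands it to its AI controller as a target.
; When PawnSensing sees a ThirdPersonCharacter, it passes that pawn to SetTarget on its DefaultAI_Melee controller.
; On possession it calls SelectAbility, which makes no actual choice and always plays the Fireball montage.
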(event `self.ReceiveBeginPlay`
  (`parent.ReceiveBeginPlay`))

(event `self.PawnSensing.OnSeePawn`
  (params (Pawn :type "Pawn Object Reference"))
  (bind _asthird_person_character (cast `/Game/Blueprints/Player/ThirdPersonCharacter` Pawn))
  (bind _asdefault_ai_melee (cast `/Game/Blueprints/Target/AI/DefaultAI_Melee` (`self.GetController`)))
  (`/Game/Blueprints/Target/AI/DefaultAI_Melee.SetTarget` _asdefault_ai_melee _asthird_person_character))

(event `self.ReceivePossessed`
  (params (NewController :type "Controller Object Reference"))
  (`self.SelectAbility`))

(fn `SelectAbility`
  (`self.PlayAnimMontage` "/Game/Animations/Fireball_Montage.Fireball_Montage"))

(fn `UserConstructionScript`
  (`parent.UserConstructionScript`))