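; Enemy fire mage that patrols a list of locations and casts fireball and curse abilities at the player.
; Pawn sensing stores the seen pawn and, through a DoOnce, spawns a fireball from the hand socket, then starts a one-shot timer that casts a curse.
; Casting-status events pause or resume that timer, with resume also restarting patrol movement.
; Player death or the target moving out of range clears the timer and target.
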(event `AIMoveEvent`
  (if (`KismetArrayLibrary.Array_IsNotEmpty` (`self.Locations`))
    (`|AIMoveTo` self (`|GetArrayItem` (`self.Locations`) (`self.StepInt`)) null
      (:`OnSuccess`
        (if (> (`self.StepInt`) (`KismetArrayLibrary.Array_Length` (`self.Locations`)))
          (set `self.StepInt` 0)
          (else
            (`/Engine/EditorBlueprintResources/StandardMacros.IncrementInt` (`self.StepInt`)
              (:`  `
                _))))
        (`self.AIMoveEvent`)))))

(event `self.ReceiveBeginPlay`
  (`parent.ReceiveBeginPlay`)
  (bind _asthird_person_character (cast `/Game/Blueprints/Player/ThirdPersonCharacter` (`GameplayStatics.GetPlayerCharacter` 0)))
  (add `self.CharacterDeath` _asthird_person_character (delegate `PlayerDeath`))
  (`self.AIMoveEvent`)
  (add `self.Can'tCastStatus` (delegate `PauseCastTimer`))
  (add `self.CanCastAgain` (delegate `UnpauseCastTimer`)))

(event `PauseCastTimer`
  (bind _fireball_timer (`self.Fireball Timer`))
  (if (`KismetSystemLibrary.K2_IsValidTimerHandle` _fireball_timer)
    (`KismetSystemLibrary.K2_PauseTimerHandle` _fireball_timer)))

(event `PlayerDeath`
  (`KismetSystemLibrary.K2_ClearAndInvalidateTimerHandle` (`self.Fireball Timer`))
  (set `self.Overlapped` null))

(event `self.ReceiveTick`
  (params (DeltaSeconds :type "Float (single-precision)"))
  (`self.Overlapped`
    (:`then`
      (bind _output_get (set `self.Distance` (`self.GetDistanceTo` (`self.Overlapped`))))
      (if (>= _output_get 2000.0)
        (`KismetSystemLibrary.K2_ClearAndInvalidateTimerHandle` (`self.Fireball Timer`))
        (set `self.Overlapped` null)))
    (:`else`)))

(event `UnpauseCastTimer`
  (`self.AIMoveEvent`)
  (if (`KismetSystemLibrary.K2_IsValidTimerHandle` (`self.Fireball Timer`))
    (`KismetSystemLibrary.K2_UnPauseTimerHandle` (struct))
    (else
      (bind _returnvalue (`KismetSystemLibrary.K2_SetTimerDelegate` (delegate `CastCurse`) 3.0 :!label _label))
      (set `self.Fireball Timer` _returnvalue))))

(event `self.PawnSensing.OnSeePawn`
  (params (Pawn :type "Pawn Object Reference"))
  (set `self.Overlapped` Pawn)
  (if (not (`KismetSystemLibrary.K2_IsValidTimerHandle` (`self.Fireball Timer`)))
    (`/Engine/EditorBlueprintResources/StandardMacros.DoOnce` false
      (:`Completed`
        (if (not (`self.StatusPreventingCasting?`))
          (`self.CastFireball`)
          (goto _label))))))

(event `CastCurse`
  (`|SpawnActorFromClass` "/Game/Blueprints/Abilities/Debuffs/Ability_Debuff_Curse.Ability_Debuff_Curse_C" (`SceneComponent.K2_GetComponentToWorld` (`self.Mesh`)) "Undefined" "OverrideRootScale" null self (`self.PlayerRef`) null))

(event `CastFireball`
  (bind _mesh (`self.Mesh`))
  (bind _asthird_person_character (cast `/Game/Blueprints/Player/ThirdPersonCharacter` (`self.Overlapped`)))
  (`|SpawnActorFromClass` "/Game/Blueprints/Abilities/Projectiles/Ability_Fireball_Remake.Ability_Fireball_Remake_C" (`SceneComponent.GetSocketTransform` _mesh (`SkinnedMeshComponent.GetSocketBoneName` _mesh "hand_rSocket") "RTS_World") "Undefined" "OverrideRootScale" null self _asthird_person_character null))

(fn `UserConstructionScript`
  (`parent.UserConstructionScript`))