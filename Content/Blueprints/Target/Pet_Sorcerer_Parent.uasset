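; Parent Blueprint for sorcerer pets, inheriting from another parent class and tied to a PetOwner.
; On BeginPlay it plays creation sound and particle, copies the owner's display level, sets HP to a third of the owner's, and determines weapon and armor strength.
; It then toggles the creation particle off and starts the persistent particle and sound.
; On Tick, when following outside combat, it turns to face its owner after a frame-length delay.
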(event `self.ReceiveBeginPlay`
  (bind _persistentsound (`self.PersistentSound`))
  (bind _petowner (`self.PetOwner`))
  (bind _creationparticle (`self.CreationParticle`))
  (bind _returnvalue (/ (`/Game/Blueprints/Character_Base_for_MMO.Total HP` _petowner) 3))
  (`parent.ReceiveBeginPlay`)
  (`SceneComponent.SetVisibility` _creationparticle true false)
  (`GameplayStatics.PlaySoundAtLocation` (`self.CreationSound`) (`self.K2_GetActorLocation` self) (struct) 1.0 1.0 0.0 null null null null)
  (set `self.DisplayLevel` (`/Game/Blueprints/Character_Base_for_MMO.DisplayLevel` _petowner))
  (set `self.Total HP` _returnvalue)
  (set `self.Current HP` _returnvalue)
  (`self.DetermineWeaponAndArmorStrength`)
  (`SceneComponent.ToggleVisibility` _creationparticle false)
  (`SceneComponent.SetVisibility` (`self.PersistentParticle`) true false)
  (`AudioComponent.SetSound` _persistentsound (`self.Persistent Sound SFX`))
  (`ActorComponent.ToggleActive` _persistentsound))

(event `self.ReceiveTick`
  (params (DeltaSeconds :type "Float (single-precision)"))
  (if (and (`self.FollowMode`) (`self.NonCombatMode`))
    (`KismetSystemLibrary.Delay` DeltaSeconds)
    (`self.K2_SetActorRotation` (`KismetMathLibrary.FindLookAtRotation` (`self.K2_GetActorLocation` self) (`self.K2_GetActorLocation` (`self.PetOwner`))))))

(fn `UserConstructionScript`
  (`parent.UserConstructionScript`))