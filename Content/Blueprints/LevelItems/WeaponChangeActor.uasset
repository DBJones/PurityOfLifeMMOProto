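; A level pickup that swaps the overlapping ThirdPersonCharacter's weapon for the configured WeaponToChange class.
; On box overlap it destroys attached Weapon_Parent actors, spawns the new weapon, stores it as CurrentWeapon and attaches it to the hand_rSocket.
; TotalWeaponStrength copies the spawned weapon's original strength, truncated.
; The weapon's strength is then overwritten from DefaultWeaponStats by the character's DisplayLevel, keeping its other details.
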(event `self.Box.OnComponentBeginOverlap`
  (params (OverlappedComponent :type "PrimitiveComponent Object Reference") (OtherActor :type "Actor Object Reference") (OtherComp :type "PrimitiveComponent Object Reference") (OtherBodyIndex :type Integer) (bFromSweep :type Boolean) (SweepResult :type "HitResult Structure (by ref)"))
  (bind _default_weapon_stats_defaultweaponstrength (break `/Game/Blueprints/Player/LevelledArmorAndWeaponData/LevelledWeaponStrength` (`self.default weapon stats`)))
  (bind _as_third_person_character (`self.As Third Person Character`))
  (bind _asthird_person_character (cast `/Game/Blueprints/Player/ThirdPersonCharacter` OtherActor))
  (bind _output_get (set `self.As Third Person Character` _asthird_person_character))
  (for _array_element (`self.GetAttachedActors` _output_get true false)
    (cast `/Game/Blueprints/Items/Weapons/Weapon_Parent` _array_element)
    (`self.K2_DestroyActor` _array_element))
  (bind _returnvalue (`|SpawnActorFromClass` (`self.WeaponToChange`) (`self.GetTransform` self) "Undefined" "OverrideRootScale" null null))
  (set `/Game/Blueprints/Player/ThirdPersonCharacter.CurrentWeapon` _returnvalue _as_third_person_character)
  (bind (_weapondetails_weaponname _weapondetails_weaponstrength _weapondetails_requiredlevel _weapondetails_acceptedspellbook _weapondetails_associatedskill _weapondetails_acceptedaugmentationrune _weapondetails_runeslot1 _weapondetails_runeslot2 _weapondetails_slot1available_ _weapondetails_slot2available_ _weapondetails_vitality _weapondetails_endurance _weapondetails_prestige _weapondetails_magicaldefense _weapondetails_physicaldefense _weapondetails_augmentationcrystalslots _weapondetails_ncrystalslots _weapondetails_bonusstats) (break `/Game/Blueprints/Items/Weapons/WeaponDetails` (`/Game/Blueprints/Items/Weapons/Weapon_Parent.WeaponDetails` _returnvalue)))
  (set `/Game/Blueprints/Character_Base_for_MMO.TotalWeaponStrength` (`KismetMathLibrary.FTrunc` _weapondetails_weaponstrength) _as_third_person_character)
  (set `/Game/Blueprints/Items/Weapons/Weapon_Parent.WeaponDetails` (make `/Game/Blueprints/Items/Weapons/WeaponDetails` _weapondetails_weaponname (`KismetMathLibrary.Conv_IntToDouble` (`BlueprintMapLibrary.Map_Find` _default_weapon_stats_defaultweaponstrength (`/Game/Blueprints/Character_Base_for_MMO.DisplayLevel` (`self.As Third Person Character`)))) _weapondetails_requiredlevel _weapondetails_acceptedspellbook _weapondetails_associatedskill _weapondetails_acceptedaugmentationrune _weapondetails_runeslot1 _weapondetails_runeslot2 _weapondetails_slot1available_ _weapondetails_slot2available_ _weapondetails_vitality _weapondetails_endurance _weapondetails_prestige _weapondetails_magicaldefense _weapondetails_physicaldefense _weapondetails_augmentationcrystalslots _weapondetails_ncrystalslots _weapondetails_bonusstats) _returnvalue)
  (`self.K2_AttachToComponent` _returnvalue (`Character.Mesh` (`self.As Third Person Character`)) "hand_rSocket" "SnapToTarget" "SnapToTarget" "SnapToTarget" true))

(fn `UserConstructionScript`)