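; A level item actor that sets the player's displayed level to its configured LevelToSet value on touch.
; At BeginPlay it shows that value on a TextRender.
; When a ThirdPersonCharacter overlaps component R, it assigns DisplayLevel, zeroes the first active skill's level, fires the level-changed call and calls that skill's LevelUpGainExp with zero experience.
; The DestroyActor node is unwired, so the item stays in the level.
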(event `self.ReceiveBeginPlay`
  (`TextRenderComponent.K2_SetText` (`self.TextRender`) (`KismetTextLibrary.Conv_IntToText` (`self.LevelToSet`))))

(event `self.r.OnComponentBeginOverlap`
  (params (OverlappedComponent :type "PrimitiveComponent Object Reference") (OtherActor :type "Actor Object Reference") (OtherComp :type "PrimitiveComponent Object Reference") (OtherBodyIndex :type Integer) (bFromSweep :type Boolean) (SweepResult :type "HitResult Structure (by ref)"))
  (bind _asthird_person_character (cast `/Game/Blueprints/Player/ThirdPersonCharacter` OtherActor))
  (set `/Game/Blueprints/Character_Base_for_MMO.DisplayLevel` (`self.LevelToSet`) _asthird_person_character)
  (bind _output (`|GetArrayItem` (`/Game/Blueprints/Player/ThirdPersonCharacter.ActiveSkills` _asthird_person_character)))
  (set `/Game/Blueprints/Skills/Skill_Parent.Level` 0 _output)
  (`/Game/Blueprints/Player/ThirdPersonCharacter.DisplayLevelChanged` _asthird_person_character)
  (`/Game/Blueprints/Skills/Skill_Parent.LevelUpGainExp` _output 0))

(fn `UserConstructionScript`)