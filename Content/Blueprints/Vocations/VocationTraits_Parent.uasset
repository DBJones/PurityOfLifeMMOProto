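; Base actor for vocation traits, with an empty ApplyEffect hook, presumably for child traits to override.
; On BeginPlay it caches the ThirdPersonCharacter player, snaps itself onto that character and prints a debug message with its name.
; It then takes the HUD reference from the PC_Mouse_Controls game mode and calls ApplyEffect, which only runs if both casts succeed.
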(event `self.ReceiveBeginPlay`
  (bind _asthird_person_character (cast `/Game/Blueprints/Player/ThirdPersonCharacter` (`GameplayStatics.GetPlayerCharacter` 0)))
  (set `self.Player Ref` _asthird_person_character)
  (`self.K2_AttachToActor` (`self.Player Ref`) "None" "SnapToTarget" "SnapToTarget" "SnapToTarget")
  (`KismetSystemLibrary.PrintString` (`KismetStringLibrary.Concat_StrStr` "Generated " (`KismetSystemLibrary.GetDisplayName` self)))
  (bind _aspc_mouse_controls (cast `/Game/Blueprints/PC_Mouse_Controls` (`GameplayStatics.GetGameMode`)))
  (set `self.Heads Up Display` (`/Game/Blueprints/PC_Mouse_Controls.Heads Up Display` _aspc_mouse_controls))
  (`self.ApplyEffect`))

(fn `ApplyEffect`)

(fn `UserConstructionScript`)