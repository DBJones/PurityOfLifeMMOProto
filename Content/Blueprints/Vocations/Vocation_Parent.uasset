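; Base actor for player vocations, registering itself as the player's current vocation on BeginPlay.
; UpdateLevel derives the vocation level from the player's SkillLevels, indexed by the ArrayInt class default of the first active skill.
; It then rebuilds traits by destroying previously spawned trait actors, spawning the TraitList class for each index up to that level, and attaching each to itself.
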(event `self.ReceiveBeginPlay`
  (bind _asthird_person_character (cast `/Game/Blueprints/Player/ThirdPersonCharacter` (`GameplayStatics.GetPlayerCharacter` 0)))
  (bind _output_get (set `self.PlayerRef` _asthird_person_character))
  (set `/Game/Blueprints/Player/ThirdPersonCharacter.CurrentVocation` self _output_get))

(event `UpdateLevel`
  (bind _playerref (`self.PlayerRef`))
  (bind _output_get (set `self.Level` (`|GetArrayItem` (`/Game/Blueprints/Player/ThirdPersonCharacter.SkillLevels` _playerref) (`.ArrayInt` (defaults `Object` (`GameplayStatics.GetObjectClass` (`|GetArrayItem` (`/Game/Blueprints/Player/ThirdPersonCharacter.ActiveSkills` _playerref))))))))
  (`self.CreateActiveTraitList` _output_get))

(fn `CreateActiveTraitList`
  (params (Level :type Integer))
  (bind _unlockedtraitlist (`self.UnlockedTraitList`))
  (bind _output_get (set `self.Level` Level))
  (if (> (`KismetArrayLibrary.Array_Length` _unlockedtraitlist) 0)
    (for _array_element _unlockedtraitlist
      (`/Engine/EditorBlueprintResources/StandardMacros.IsValid` _array_element
        (:`Is Valid`
          (`self.K2_DestroyActor` _array_element)))))
  (for _index (range (+ _output_get 1))
    (bind _returnvalue (`|SpawnActorFromClass` (`BlueprintMapLibrary.Map_Find` (`self.TraitList`) _index) (`self.GetTransform` self) "AlwaysSpawn" "OverrideRootScale" null null))
    (`/Engine/EditorBlueprintResources/StandardMacros.IsValid` _returnvalue
      (:`Is Valid`
        (`KismetArrayLibrary.Array_Add` (`self.UnlockedTraitList`) _returnvalue)
        (`self.K2_AttachToActor` _returnvalue self "None" "SnapToTarget" "SnapToTarget" "SnapToTarget" true)))))

(fn `UserConstructionScript`)