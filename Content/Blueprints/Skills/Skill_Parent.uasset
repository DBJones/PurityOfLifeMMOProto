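; Base skill Blueprint that tracks unlock state, level and accumulated EXP for a player skill.
; An unlock event sets the starting level, and per-level EXP costs follow a power-times-log curve summed into a cumulative threshold.
; Gaining EXP raises at most one level per call up to the cap, then updates the player's skill array, stats and current vocation level and fires an EXP-gained call.
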(event `self.ReceiveBeginPlay`
  (add `self.SkillUnlocked` (delegate `UnlockSkill`))
  (bind _asthird_person_character (cast `/Game/ThirdPersonBP/Blueprints/Player/ThirdPersonCharacter` (`GameplayStatics.GetPlayerCharacter` 0)))
  (set `self.PlayerRef` _asthird_person_character))

(event `UnlockSkill`
  (bind _unlocklevel (`self.UnlockLevel`))
  (set `self.Unlocked?` true)
  (set `self.Level` _unlocklevel)
  (bind _outexp (`self.CaluclateEXPToNextLevel` _unlocklevel))
  (set `self.EXPToNextLevel` _outexp)
  (`self.CalculateEXPSumToNextLevel` 0)
  (`self.CalculateEXPToNextLevel` (`self.EXPAccumulated`)))

(fn `CalculateEXPSumToNextLevel`
  (params (Level :type Integer))
  (set `self.EXPTotalToNextLevel` 0)
  (for _index (range 1 (+ (`KismetMathLibrary.Clamp` Level 1 (`self.LevelCap`)) 1))
    (bind _outexp (`self.CaluclateEXPToNextLevel` _index))
    (set `self.EXPTotalToNextLevel` (+ _outexp (`self.EXPTotalToNextLevel`)))))

(fn `CalculateEXPToNextLevel`
  (params (CurrentXPTotal :type Integer))
  (returns (OutputEXP :type Integer))
  (return (- (`self.EXPTotalToNextLevel`) CurrentXPTotal)))

(fn `CaluclateEXPToNextLevel`
  (params (InInt :type Integer))
  (returns (OutExp :type Integer))
  (return (`KismetMathLibrary.FTrunc` (* (`KismetMathLibrary.MultiplyMultiply_FloatFloat` (`KismetMathLibrary.Conv_IntToDouble` InInt) 1.3) (`KismetMathLibrary.Loge` (* (`KismetMathLibrary.Conv_IntToDouble` InInt) 1.4)) 210.0))))

(fn `LevelUpGainExp`
  (params (EXPGained :type Integer))
  (bind _level (`self.Level`))
  (bind _level_2 (`self.Level`))
  (bind _playerref (`self.PlayerRef`))
  (if (< (`self.Level`) (`self.LevelCap`))
    (bind _output_get (set `self.EXPAccumulated` (+ EXPGained (`self.EXPAccumulated`))))
    (if (>= _output_get (`self.EXPTotalToNextLevel`))
      (`/Engine/EditorBlueprintResources/StandardMacros.IncrementInt` _level_2
        (:`  `
          (bind _outputexp (`self.CalculateEXPToNextLevel` (`self.EXPAccumulated`)))
          (set `self.EXPToNextLevel` _outputexp)))))
  (`self.CalculateEXPSumToNextLevel` _level_2)
  (set `/Game/ThirdPersonBP/Blueprints/Player/ThirdPersonCharacter.Display Level` _level _playerref)
  (`KismetArrayLibrary.Array_Set` (`/Game/ThirdPersonBP/Blueprints/Player/ThirdPersonCharacter.SkillLevels` _playerref) (`self.ArrayInt`) _level)
  (`/Game/ThirdPersonBP/Blueprints/Player/ThirdPersonCharacter.RecalculateStats` _playerref)
  (`/Game/ThirdPersonBP/Blueprints/Vocations/Vocation_Parent.UpdateLevel` (`/Game/ThirdPersonBP/Blueprints/Player/ThirdPersonCharacter.CurrentVocation` _playerref))
  (`self.EXPGained`))

(fn `UserConstructionScript`)