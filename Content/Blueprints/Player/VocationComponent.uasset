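; Player component that spawns and switches the active Vocation actor, attached to the component's owner.
; GenerateVocationActor checks the class in the VocationUnlockStatus map; an unlocked, different class replaces and destroys CurrentVocation.
; A locked class is spawned as CurrentVocation without destroying the previous actor.
; Its unlock flag is set only on an array copied from the map's values, so the map itself stays unchanged.
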(fn `GenerateVocationActor`
  (params (VocationToCreate :type "/Game/Blueprints/Vocations/Vocation_Parent Class Reference") (Transform :type "Transform Structure"))
  (bind _currentvocation (`self.CurrentVocation`))
  (bind _vocationunlockstatus (`self.VocationUnlockStatus`))
  (if (`BlueprintMapLibrary.Map_Find` (`self.VocationUnlockStatus`) VocationToCreate)
    (if (not (== (`GameplayStatics.GetObjectClass` _currentvocation) VocationToCreate))
      (`Actor.K2_DestroyActor` _currentvocation)
      (bind _returnvalue (`|SpawnActorFromClass` (`local.VocationToCreate`) (`local.Transform`) "Undefined" "OverrideRootScale" null null))
      (`Actor.K2_AttachToActor` _returnvalue (`self.GetOwner` self) "None" "SnapToTarget" "SnapToTarget" "SnapToTarget" true)
      (set `self.CurrentVocation` _returnvalue))
    (else
      (bind _keys (`BlueprintMapLibrary.Map_Keys` _vocationunlockstatus))
      (bind _values (`BlueprintMapLibrary.Map_Values` _vocationunlockstatus))
      (`KismetArrayLibrary.Array_Set` _values (`KismetArrayLibrary.Array_Find` _keys (`local.VocationToCreate`)) true)
      (bind _returnvalue_2 (`|SpawnActorFromClass` (`local.VocationToCreate`) (`local.Transform`) "Undefined" "OverrideRootScale" null null))
      (`Actor.K2_AttachToActor` _returnvalue_2 (`self.GetOwner`) "None" "SnapToTarget" "SnapToTarget" "SnapToTarget" true)
      (set `self.CurrentVocation` _returnvalue_2))))