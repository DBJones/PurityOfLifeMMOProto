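; Player skill component that spawns and swaps the owner's active weapon skill actor for an MMO character.
; GenerateSkillActor replaces a differing skill if unlocked, otherwise spawns it at its default UnlockLevel, then attaches it and copies its level to the character's DisplayLevel.
; Unlock, active and level updates write to arrays from map Values(), with no write-back to the maps.
; The active-skill OnRep handler is empty.
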(fn `GenerateSkillActor`
  (params (SkillToBeGeneratedParent :type "/Game/Blueprints/Skills/Skill_Parent Class Reference") (Transform :type "Transform Structure"))
  (returns (SkillGenerated :type "/Game/Blueprints/Skills/Skill_Parent Object Reference"))
  (bind _skill_activestatus (`self.Skill_ActiveStatus`))
  (bind _activeweaponskill (`self.ActiveWeaponSkill`))
  (bind _skilltobegeneratedparent (`local.SkillToBeGeneratedParent`))
  (bind _skill_unlockedstatus (`self.Skill_UnlockedStatus`))
  (bind _levels (`self.Levels`))
  (bind _skill_activestatus_2 (`self.Skill_ActiveStatus`))
  (bind _returnvalue (`self.GetOwner` self))
  (bind _returnvalue_2 (`GameplayStatics.GetObjectClass` _activeweaponskill))
  (bind _returnvalue_3 (`self.GetOwner` self))
  (bind (_name _level _acceptedweapons _expaccumulated _exptonextlevel _exptotaltonextlevel _arrayint _unlocked_ _skillunlocked _unlocklevel) (defaults `Object` _skilltobegeneratedparent))
  (if (`BlueprintMapLibrary.Map_Find` (`self.Skill_UnlockedStatus`) SkillToBeGeneratedParent)
    (if (not (== _returnvalue_2 SkillToBeGeneratedParent))
      (bind _keys (`BlueprintMapLibrary.Map_Keys` _skill_activestatus))
      (bind _values (`BlueprintMapLibrary.Map_Values` _skill_activestatus))
      (`KismetArrayLibrary.Array_Set` _values (`KismetArrayLibrary.Array_Find` _keys _returnvalue_2))
      (`Actor.K2_DestroyActor` _activeweaponskill)
      (bind _returnvalue_4 (`|SpawnActorFromClass` (`local.SkillToBeGeneratedParent`) (`local.Transform`) "Undefined" "OverrideRootScale" null null))
      (`Actor.K2_AttachToActor` _returnvalue_4 _returnvalue "None" "SnapToTarget" "SnapToTarget" "SnapToTarget" true)
      (bind _output_get (set `self.ActiveWeaponSkill` _returnvalue_4))
      (bind _output_get_2 (set `/Game/Blueprints/Skills/Skill_Parent.Level` (`BlueprintMapLibrary.Map_Find` (`self.Levels`) (`local.SkillToBeGeneratedParent`)) _output_get))
      (bind _ascharacter_base_for_mmo (cast `/Game/Blueprints/Character_Base_for_MMO` _returnvalue))
      (set `/Game/Blueprints/Character_Base_for_MMO.DisplayLevel` _output_get_2 _ascharacter_base_for_mmo)
      (return _output_get))
    (else
      (bind _keys_2 (`BlueprintMapLibrary.Map_Keys` _skill_unlockedstatus))
      (bind _values_2 (`BlueprintMapLibrary.Map_Values` _skill_unlockedstatus))
      (`KismetArrayLibrary.Array_Set` _values_2 (`KismetArrayLibrary.Array_Find` _keys_2 (`local.SkillToBeGeneratedParent`)) true)
      (bind _keys_3 (`BlueprintMapLibrary.Map_Keys` _levels))
      (bind _values_3 (`BlueprintMapLibrary.Map_Values` _levels))
      (`KismetArrayLibrary.Array_Set` _values_3 (`|GetArrayItem` _values_3 (`KismetArrayLibrary.Array_Find` _keys_3 _skilltobegeneratedparent)) _unlocklevel)
      (bind _returnvalue_5 (`|SpawnActorFromClass` (`local.SkillToBeGeneratedParent`) (`local.Transform`) "Undefined" "OverrideRootScale" null null))
      (`Actor.K2_AttachToActor` _returnvalue_5 _returnvalue_3 "None" "SnapToTarget" "SnapToTarget" "SnapToTarget" true)
      (bind _output_get_3 (set `self.ActiveWeaponSkill` _returnvalue_5))
      (bind _output_get_4 (set `/Game/Blueprints/Skills/Skill_Parent.Level` _unlocklevel _output_get_3))
      (bind _ascharacter_base_for_mmo_2 (cast `/Game/Blueprints/Character_Base_for_MMO` _returnvalue_3))
      (set `/Game/Blueprints/Character_Base_for_MMO.DisplayLevel` _output_get_4 _ascharacter_base_for_mmo_2)
      (bind _keys_4 (`BlueprintMapLibrary.Map_Keys` _skill_activestatus_2))
      (bind _values_4 (`BlueprintMapLibrary.Map_Values` _skill_activestatus_2))
      (`KismetArrayLibrary.Array_Set` _values_4 (`KismetArrayLibrary.Array_Find` _keys_4 (`local.SkillToBeGeneratedParent`)) true)
      (return _output_get_3))))

(fn `OnRep_ActiveSkill`)