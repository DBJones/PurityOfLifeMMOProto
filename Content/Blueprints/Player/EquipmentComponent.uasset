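; Player equipment component that spawns weapons and puts them in the character's hand.
; SpawnWeaponFromClass spawns the given class, attaches it to the ThirdPersonCharacter owner's mesh at the right-hand socket with world rotation kept, and stores it as CurrentWeapon.
; It prints a debug string and returns the SkillTrained value from the weapon's class defaults.
; The owner cast follows the spawn, so a failed cast leaves the weapon unattached.
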(fn `SpawnWeaponFromClass`
  (params (WeaponClass :type "/Game/Blueprints/Items/Weapons/Weapon_Parent Class Reference") (SpawnTransform :type "Transform Structure"))
  (returns (SkillTrained :type "/Game/Blueprints/Skills/Skill_Parent Class Reference"))
  (bind _returnvalue (`|SpawnActorFromClass` WeaponClass SpawnTransform "Undefined" "OverrideRootScale" null null))
  (bind _asthird_person_character (cast `/Game/Blueprints/Player/ThirdPersonCharacter` (`self.GetOwner` self)))
  (`Actor.K2_AttachToComponent` _returnvalue (`Character.Mesh` _asthird_person_character) "hand_rSocket" "SnapToTarget" "KeepWorld" "SnapToTarget" true)
  (set `self.CurrentWeapon` _returnvalue)
  (`KismetSystemLibrary.PrintString` "Hello" true true (struct :`G` 0.66 :`B` 1.0 :`A` 1.0) 20.0)
  (return (`.SkillTrained` (defaults `Object` (`GameplayStatics.GetObjectClass` _returnvalue)))))