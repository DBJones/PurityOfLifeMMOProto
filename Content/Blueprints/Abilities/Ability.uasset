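; Base spell/skill actor attached to the caster's hand, with an empty ActivateEffect that the HUD cast bar's success event triggers.
; For player casters, BeginPlay applies trait cost changes, then validates target, range and resources before casting or interrupting.
; Energy Conversion swaps mana and stamina costs at a premium.
; Helpers compute stat-based damage and healing with random crits, route damage through shields, roll status effects and look up weapon-rune bonuses.
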(event `self.ReceiveBeginPlay`
  (bind (_ability_details_name _ability_details_description _ability_details_levelreq _ability_details_manacost _ability_details_staminacost _ability_details_cooldown _ability_details_casttime _ability_details_basepower _ability_details_isinterruptible _ability_details_icon _ability_details_tags _ability_details_validtargetlist _ability_details_healingspell_ _ability_details_range) (break `/Game/Blueprints/Abilities/AbilityDetails` (`self.Ability Details`)))
  (bind _caster (`self.Caster`))
  (switch `/Game/Blueprints/Abilities/TargetRange` _ability_details_range
    (:`NewEnumerator0`
      (set `self.RangeCalcFromEnum` 1200.0))
    (:`NewEnumerator1`
      (set `self.RangeCalcFromEnum` 600.0))
    (:`NewEnumerator2`
      (set `self.RangeCalcFromEnum` 300.0))
    (:`NewEnumerator3`
      (set `self.RangeCalcFromEnum` 50.0)))
  (bind _asthird_person_character (cast `/Game/Blueprints/Player/ThirdPersonCharacter` (`GameplayStatics.GetPlayerCharacter` 0)))
  (set `self.PlayerRef` _asthird_person_character)
  (`self.K2_AttachToComponent` (`Character.Mesh` _caster) "hand_rSocket" "SnapToTarget" "SnapToTarget" "SnapToTarget")
  (if (== (`GameplayStatics.GetObjectClass` _caster) "/Game/Blueprints/Player/ThirdPersonCharacter.ThirdPersonCharacter_C")
    (`self.UpdateCosts`)
    (`/Game/Blueprints/Player/ThirdPersonCharacter.CheckLastAbility` (`self.PlayerRef`) self)
    (bind _asmouse_controller (cast `/Game/Blueprints/Mouse_Controller` (`GameplayStatics.GetPlayerController` 0)))
    (bind _output_get (set `self.Heads Up Display` (`/Game/Blueprints/Mouse_Controller.W_HUD` _asmouse_controller)))
    (add `/Game/Blueprints/UI/UI_ActionBar/CastBar_UI.CastSuccessful` (`/Game/Blueprints/UI/HeadsUpDisplay.CastBar_UI` _output_get) (delegate `Active`))
    (bind _validtarget_ (`self.CheckTarget`))
    (if _validtarget_
      (if (`/Game/Blueprints/Character_Base_for_MMO.IsCasting?` (`self.Caster`))
        (`KismetSystemLibrary.PrintString` "Cannot Cast while Casting")
        (`self.InterruptCast`)
        (else
          (set `/Game/Blueprints/Character_Base_for_MMO.IsCasting?` true _caster)
          (`self.BeginCasting`)))
      (else
        (`KismetSystemLibrary.PrintString` "Invalid Target")
        (`self.InterruptCast`)))))

(event `Active`
  (`self.ActivateEffect`))

(event `SuccessfulCast`
  (bind _caster (`self.Caster`))
  (bind _playerref (`self.PlayerRef`))
  (bind _sfxcastingcomponent (`self.SFXCastingComponent`)
    (:`then`
      (`ActorComponent.SetActive` _sfxcastingcomponent false false))
    (:`else`
      _))
  (set `/Game/Blueprints/Character_Base_for_MMO.IsCasting?` false _caster)
  (if (== _playerref _caster)
    (`/Game/Blueprints/Player/ThirdPersonCharacter.ReadyToCastAgain` _playerref))
  (`KismetSystemLibrary.Delay` 0.1)
  (`self.CastSuccess`))

(fn `ActivateEffect`)

(fn `BeginCasting`
  (bind (_ability_details_name _ability_details_description _ability_details_levelreq _ability_details_manacost _ability_details_staminacost) (break `/Game/Blueprints/Abilities/AbilityDetails` (`self.Ability Details`)))
  (bind _caster (`self.Caster`))
  (bind _ability_details (`self.Ability Details`))
  (if (and (> (`self.GetDistanceTo` (`self.Target`) (`self.Caster`)) (`self.RangeCalcFromEnum`)) (not (`.AffectsSelf?_5_4E2F6BCF41F5B1ABAE22379B9B2EDC3F` (break `/Game/Blueprints/Abilities/ValidTargetList` (`.ValidTargetList_32_5D30CE1541306726CB193C9368962425` (break `/Game/Blueprints/Abilities/AbilityDetails` _ability_details))))))
    (`KismetSystemLibrary.PrintString` "Too Far Away!")
    (`self.InterruptCast`)
    (else
      (`/Game/Blueprints/Character_Base_for_MMO.Casting` _caster)
      (bind _asthird_person_character (cast `/Game/Blueprints/Player/ThirdPersonCharacter` _caster))
      (set `/Game/Blueprints/Player/ThirdPersonCharacter.CurrentAbilityUsing` self _asthird_person_character)
      (if (`/Game/Blueprints/Player/ThirdPersonCharacter.EnergyConversionActive?` _asthird_person_character)
        (bind _success (`/Game/Blueprints/Player/ThirdPersonCharacter.Check Resources` _asthird_person_character (* _ability_details_staminacost 1.5) (* _ability_details_manacost 1.5)))
        (if _success
          (if (> (`.CastTime_11_4398D9B847A4C38D10E5FABE672ED33A` (break `/Game/Blueprints/Abilities/AbilityDetails` _ability_details)) 0.0) :!label _label
            (`/Game/Blueprints/UI/HeadsUpDisplay.DisplayCastBar` (`self.Heads Up Display`) self))
          (bind _castingsfx (`self.CastingSFX`)
            (:`then`
              (bind _returnvalue (`GameplayStatics.SpawnSoundAtLocation` _castingsfx (`self.K2_GetActorLocation` self) (struct) 1.0 1.0 0.0 null null))
              (bind _output_get (set `self.SFXCastingComponent` _returnvalue))
              (`ActorComponent.SetActive` _output_get true false))
            (:`else`
              _))
          (`self.CastAbility`)
          (else
            (`self.InterruptCast` :!label _label_2)))
        (else
          (bind _success_2 (`/Game/Blueprints/Player/ThirdPersonCharacter.Check Resources` _asthird_person_character (`.ManaCost_24_CDA4AD47488A20220155939F5ADB7A1B` (break `/Game/Blueprints/Abilities/AbilityDetails` _ability_details)) (`.StaminaCost_26_0A40C63B403834A1614C5EB3261A24BF` (break `/Game/Blueprints/Abilities/AbilityDetails` _ability_details))))
          (if _success_2
            (goto _label)
            (else
              (goto _label_2))))))))

(fn `CaculateRNG`
  (returns (Mult :type "Float (double-precision)"))
  (bind _returnvalue (`KismetMathLibrary.RandomFloatInRange` 0.87 1.05))
  (bind _asthird_person_character (cast `/Game/Blueprints/Player/ThirdPersonCharacter` (`self.Caster`))
    (:`then`
      (if (<= (* (`/Game/Blueprints/Player/ThirdPersonCharacter.CritRate Mult` _asthird_person_character) (`KismetMathLibrary.RandomFloatInRange` 0.0 1.0)) 0.125)
        (`self.CritMade`)
        (return (* 1.5 _returnvalue))
        (else
          (return _returnvalue))))
    (:`CastFailed`
      (return (`KismetMathLibrary.RandomFloatInRange` 1.05 1.5)))))

(fn `CalculateDamage`
  (params (ActiveAugmentationMult :type "Float (double-precision)"))
  (returns (OutDamage :type "Float (double-precision)"))
  (bind (_ability_details_name _ability_details_description _ability_details_levelreq _ability_details_manacost _ability_details_staminacost _ability_details_cooldown _ability_details_casttime _ability_details_basepower _ability_details_isinterruptible _ability_details_icon _ability_details_tags) (break `/Game/Blueprints/Abilities/AbilityDetails` (`self.Ability Details`)))
  (bind _hasshield_ (`/Game/Blueprints/Character_Base_for_MMO.HasShield?` (`self.Target`)))
  (bind _caster (`self.Caster`)
    (:`then`
      (bind _target (`self.Target`)
        (:`then`
          (bind _mult (`self.CaculateRNG`))
          (bind _outinfo (`/Game/Blueprints/Character_Base_for_MMO.CalculateLevelMult` _caster))
          (if (`BlueprintGameplayTagLibrary.DoesContainerMatchTagQuery` _ability_details_tags (`BlueprintGameplayTagLibrary.MakeGameplayTagQuery` (struct :`TagDictionary` (struct :`(TagName` "Magic")) :`QueryTokenStream` "(0,1,2,1,0)" :`AutoDescription` " ALL( Magic )")))
            (bind _magical_damage_mult (`/Game/Blueprints/Character_Base_for_MMO.Magical Damage Mult` _caster))
            (`KismetSystemLibrary.PrintString` (`KismetStringLibrary.Conv_DoubleToString` _magical_damage_mult))
            (bind _totalweaponstrength (`/Game/Blueprints/Character_Base_for_MMO.TotalWeaponStrength` _caster))
            (bind _total_resillience (`/Game/Blueprints/Character_Base_for_MMO.Total Resillience` _target))
            (bind _damagereductionmult (`/Game/Blueprints/Character_Base_for_MMO.DamageReductionMult` _target))
            (bind _returnvalue (`KismetMathLibrary.Conv_IntToDouble` (`KismetMathLibrary.FTrunc` (/ (* _mult _outinfo (`KismetMathLibrary.MultiplyMultiply_FloatFloat` (* _ability_details_basepower ActiveAugmentationMult) 1.1) _magical_damage_mult (/ (+ (`KismetMathLibrary.Conv_IntToDouble` _totalweaponstrength) (`KismetMathLibrary.Conv_IntToDouble` (`/Game/Blueprints/Character_Base_for_MMO.TotalIntelligence` _caster))) 2.5) ActiveAugmentationMult) (* (/ (+ (`KismetMathLibrary.Conv_IntToDouble` (`/Game/Blueprints/Character_Base_for_MMO.Total Magical Defense` _target)) _total_resillience) 2.0) _damagereductionmult)))))
            (if (< _returnvalue 1.0)
              (return 1.0)
              (elif _hasshield_
                (`self.DamageBarrier` _returnvalue self)
                (else
                  (return _returnvalue))))
            (else
              (bind _returnvalue_2 (`KismetMathLibrary.Conv_IntToDouble` (`KismetMathLibrary.FTrunc` (/ (* _outinfo _mult (`KismetMathLibrary.MultiplyMultiply_FloatFloat` _ability_details_basepower 1.1) (/ (+ (`KismetMathLibrary.Conv_IntToDouble` _totalweaponstrength) (`KismetMathLibrary.Conv_IntToDouble` (`/Game/Blueprints/Character_Base_for_MMO.TotalWillpower` _caster))) 2.0) (`/Game/Blueprints/Character_Base_for_MMO.Physical Damage Mult` _caster) ActiveAugmentationMult) (* (/ (+ (`KismetMathLibrary.Conv_IntToDouble` (`/Game/Blueprints/Character_Base_for_MMO.Total Physical Defense` _target)) _total_resillience) 2.0) _damagereductionmult)))))
              (if (< _returnvalue_2 1.0)
                (return 1.0)
                (elif _hasshield_
                  (`self.DamageBarrier` _returnvalue_2 self)
                  (else
                    (return _returnvalue_2)))))))
        (:`else`
          (`self.K2_DestroyActor` :!label _label))))
    (:`else`
      (goto _label))))

(fn `CalculateHealStrength`
  (params (ActiveAugmentationMult :type "Float (double-precision)"))
  (returns (HealNumber :type "Float (double-precision)"))
  (bind (_ability_details_name _ability_details_description _ability_details_levelreq _ability_details_manacost _ability_details_staminacost _ability_details_cooldown _ability_details_casttime _ability_details_basepower) (break `/Game/Blueprints/Abilities/AbilityDetails` (`self.Ability Details`)))
  (bind _caster (`self.Caster`))
  (bind _outinfo (`/Game/Blueprints/Character_Base_for_MMO.CalculateLevelMult` _caster))
  (bind _mult (`self.CaculateRNG`))
  (return (`KismetMathLibrary.Conv_IntToDouble` (`KismetMathLibrary.FTrunc` (/ (* _mult _outinfo (`KismetMathLibrary.Sqrt` (+ (`KismetMathLibrary.Conv_IntToDouble` (`/Game/Blueprints/Character_Base_for_MMO.TotalWeaponStrength` _caster)) (`KismetMathLibrary.Conv_IntToDouble` (`/Game/Blueprints/Character_Base_for_MMO.InnerGlow` _caster)))) (`/Game/Blueprints/Character_Base_for_MMO.Healing Damage Mult` _caster) (`KismetMathLibrary.MultiplyMultiply_FloatFloat` _ability_details_basepower 1.1) ActiveAugmentationMult) -150.0)))))

(fn `CastAbility`
  (bind (_ability_details_name _ability_details_description _ability_details_levelreq _ability_details_manacost _ability_details_staminacost) (break `/Game/Blueprints/Abilities/AbilityDetails` (`self.Ability Details`)))
  (bind (_ability_details_name_2 _ability_details_description_2 _ability_details_levelreq_2 _ability_details_manacost_2 _ability_details_staminacost_2) (break `/Game/Blueprints/Abilities/AbilityDetails` (`self.Ability Details`)))
  (bind _asthird_person_character (cast `/Game/Blueprints/Player/ThirdPersonCharacter` (`self.Caster`)))
  (if (`/Game/Blueprints/Player/ThirdPersonCharacter.EnergyConversionActive?` _asthird_person_character)
    (`/Game/Blueprints/Player/ThirdPersonCharacter.SpendResources` _asthird_person_character (* _ability_details_staminacost 1.5) (* _ability_details_manacost 1.5))
    (else
      (`/Game/Blueprints/Player/ThirdPersonCharacter.SpendResources` _asthird_person_character _ability_details_manacost_2 _ability_details_staminacost_2))))

(fn `CheckTarget`
  (returns (`ValidTarget?` :type Boolean) (OutTarget :type "Character Object Reference"))
  (bind _ability_details (`self.Ability Details`))
  (if (and (not (break `/Game/Blueprints/Abilities/ValidTargetList` (`.ValidTargetList_32_5D30CE1541306726CB193C9368962425` (break `/Game/Blueprints/Abilities/AbilityDetails` _ability_details)))) (not (`.AffectsEnemy?_3_62F70C3D4DBBDEC18C7024881ADB3EAC` (break `/Game/Blueprints/Abilities/ValidTargetList` (`.ValidTargetList_32_5D30CE1541306726CB193C9368962425` (break `/Game/Blueprints/Abilities/AbilityDetails` _ability_details))))) (`.AffectsSelf?_5_4E2F6BCF41F5B1ABAE22379B9B2EDC3F` (break `/Game/Blueprints/Abilities/ValidTargetList` (`.ValidTargetList_32_5D30CE1541306726CB193C9368962425` (break `/Game/Blueprints/Abilities/AbilityDetails` _ability_details)))))
    _
    (elif (and (`.AffectsSelf?_5_4E2F6BCF41F5B1ABAE22379B9B2EDC3F` (break `/Game/Blueprints/Abilities/ValidTargetList` (`.ValidTargetList_32_5D30CE1541306726CB193C9368962425` (break `/Game/Blueprints/Abilities/AbilityDetails` _ability_details)))) (`.AffectsEnemy?_3_62F70C3D4DBBDEC18C7024881ADB3EAC` (break `/Game/Blueprints/Abilities/ValidTargetList` (`.ValidTargetList_32_5D30CE1541306726CB193C9368962425` (break `/Game/Blueprints/Abilities/AbilityDetails` _ability_details)))))
      (bind _target (`self.Target`)
        (:`then`
          (if (!= (`/Game/Blueprints/Character_Base_for_MMO.Team` (`self.Caster`)) (`/Game/Blueprints/Character_Base_for_MMO.Team` (`self.Target`)))
            (return true _target)
            (else
              _)))
        (:`else`
          _))
      (elif (and (break `/Game/Blueprints/Abilities/ValidTargetList` (`.ValidTargetList_32_5D30CE1541306726CB193C9368962425` (break `/Game/Blueprints/Abilities/AbilityDetails` _ability_details))) (`.AffectsSelf?_5_4E2F6BCF41F5B1ABAE22379B9B2EDC3F` (break `/Game/Blueprints/Abilities/ValidTargetList` (`.ValidTargetList_32_5D30CE1541306726CB193C9368962425` (break `/Game/Blueprints/Abilities/AbilityDetails` _ability_details)))))
        (`self.Target`
          (:`then`
            (if (== (`/Game/Blueprints/Character_Base_for_MMO.Team` (`self.Caster`)) (`/Game/Blueprints/Character_Base_for_MMO.Team` (`self.Target`)))
              (return true _target)
              (else
                _)))
          (:`else`
            _))
        (else
          (bind _target_2 (`self.Target`)
            (:`then`
              (if (and (!= (`/Game/Blueprints/Character_Base_for_MMO.Team` (`self.Caster`)) (`/Game/Blueprints/Character_Base_for_MMO.Team` (`self.Target`))) (`.AffectsEnemy?_3_62F70C3D4DBBDEC18C7024881ADB3EAC` (break `/Game/Blueprints/Abilities/ValidTargetList` (`.ValidTargetList_32_5D30CE1541306726CB193C9368962425` (break `/Game/Blueprints/Abilities/AbilityDetails` (`self.Ability Details`))))))
                _
                (elif (and (== (`/Game/Blueprints/Character_Base_for_MMO.Team` (`self.Caster`)) (`/Game/Blueprints/Character_Base_for_MMO.Team` (`self.Target`))) (break `/Game/Blueprints/Abilities/ValidTargetList` (`.ValidTargetList_32_5D30CE1541306726CB193C9368962425` (break `/Game/Blueprints/Abilities/AbilityDetails` (`self.Ability Details`)))))
                  _
                  (else
                    (return false _target_2))))
              (return true _target_2))
            (:`else`
              (return false null)))))))
  (bind _output_get (set `self.Target` (`self.Caster`)))
  (return true _output_get))

(fn `DamageBarrier`
  (params (`Input Damage` :type "Float (double-precision)") (Ability :type "/Game/Blueprints/Abilities/Ability Object Reference"))
  (locals (Remainder :type "Float (double-precision)") (InputDamage :type "Float (double-precision)") (AbilityRef :type "/Game/Blueprints/Abilities/Ability Object Reference"))
  (bind _target (`/Game/Blueprints/Abilities/Ability.Target` Ability))
  (bind _listofactiveshields (`/Game/Blueprints/Character_Base_for_MMO.ListOfActiveShields` _target))
  (bind _output (`|GetArrayItem` _listofactiveshields))
  (bind _returnvalue (- (`/Game/Blueprints/Character_Base_for_MMO.MagicShieldHP` _target) (`local.InputDamage`)))
  (bind _returnvalue_2 (- (`/Game/Blueprints/Abilities/StatusEffects/Status_Parent.ShieldHP` _output) 0.0))
  (set `local.InputDamage` `Input Damage`)
  (if (> (`KismetArrayLibrary.Array_Length` _listofactiveshields) 1)
    (set `local.Remainder` (`local.InputDamage`))
    (if (<= _returnvalue_2 0.0) :!label _label
      (`/Game/Blueprints/Character_Base_for_MMO.MagicShieldDestroyed` _target)
      (set `local.Remainder` (`KismetMathLibrary.Abs` _returnvalue_2))
      (if (> (`KismetArrayLibrary.Array_Length` _listofactiveshields) 0)
        (goto _label)
        (else
          (`GameplayStatics.ApplyDamage` _target (`local.Remainder`) null Ability (`/Game/Blueprints/Abilities/Ability.DamageClass` Ability) :!label _label_2)))
      (else
        (set `/Game/Blueprints/Abilities/StatusEffects/Status_Parent.ShieldHP` _returnvalue_2 _output)
        (`/Game/Blueprints/Character_Base_for_MMO.MagicShieldDamaged` _target)))
    (elif (<= _returnvalue 0.0)
      (`/Game/Blueprints/Character_Base_for_MMO.MagicShieldDestroyed` _target)
      (`KismetArrayLibrary.Array_Clear` _listofactiveshields)
      (set `local.Remainder` (`KismetMathLibrary.Abs` _returnvalue))
      (goto _label_2)
      (else
        (set `/Game/Blueprints/Character_Base_for_MMO.MagicShieldHP` _returnvalue _target)))))

(fn `Determine Augmentation Benefit`
  (params (Caster :type "Character Object Reference") (DamageClass :type "DamageType Class Reference"))
  (returns (OutAugmentationMult :type "Float (double-precision)"))
  (bind _playerref (`self.PlayerRef`))
  (bind (_weapondetails_weaponname _weapondetails_weaponstrength _weapondetails_requiredlevel _weapondetails_acceptedspellbook _weapondetails_associatedskill _weapondetails_acceptedaugmentationrune _weapondetails_runeslot1 _weapondetails_runeslot2) (break `/Game/Blueprints/Items/Weapons/WeaponDetails` (`/Game/Blueprints/Items/Weapons/Weapon_Parent.WeaponDetails` (`/Game/Blueprints/Character_Base_for_MMO.CurrentWeapon` _playerref))))
  (if (== Caster _playerref)
    (bind _outarrayofmults (`/Game/Blueprints/Player/ThirdPersonCharacter.CalculateAugmentationBonuses` _playerref))
    (`/Engine/EditorBlueprintResources/StandardMacros.IsValid` _weapondetails_runeslot1
      (:`Is Valid`
        (if (== DamageClass (`/Game/Blueprints/Items/AugmentationRunes/Augmentation_Rune_Parent.CorrespDmgActor` _weapondetails_runeslot1))
          (return (`|GetArrayItem` _outarrayofmults 1))
          (else
            _)))
      (:`Is Not Valid`
        _))
    (`/Engine/EditorBlueprintResources/StandardMacros.IsValid` _weapondetails_runeslot2
      (:`Is Valid`
        (if (== DamageClass (`/Game/Blueprints/Items/AugmentationRunes/Augmentation_Rune_Parent.CorrespDmgActor` _weapondetails_runeslot2))
          (return (`|GetArrayItem` _outarrayofmults 2))
          (else
            _)))
      (:`Is Not Valid`
        _))
    (return (`|GetArrayItem` _outarrayofmults))
    (else
      (return 1.0))))

(fn `InterruptCast`
  (bind _sfxcastingcomponent (`self.SFXCastingComponent`)
    (:`then`
      (`ActorComponent.SetActive` _sfxcastingcomponent false false))
    (:`else`
      _))
  (`GameplayStatics.PlaySound2D` (`self.InterruptSFX`) 0.8 2.0 0.0 null null)
  (set `/Game/Blueprints/Character_Base_for_MMO.IsCasting?` false (`self.Caster`))
  (`self.CastInterrupted`)
  (`self.K2_DestroyActor`))

(fn `SpawnStatus`
  (bind _target (`self.Target`))
  (for (_array_element _array_index) (`self.StatusEffects`)
    (if (<= (`KismetMathLibrary.RandomFloatInRange` 0.0 100.0) (`|GetArrayItem` (`self.PercentChancesForEach`) _array_index))
      (bind _returnvalue (`|SpawnActorFromClass` _array_element (`self.GetTransform` self) "Undefined" "OverrideRootScale" null _target (`self.Caster`) 5.0 0.0 null))
      (`/Engine/EditorBlueprintResources/StandardMacros.IsValid` _returnvalue
        (:`Is Valid`
          (`self.K2_AttachToActor` _returnvalue _target "hand_rSocket" "SnapToTarget" "SnapToTarget" "SnapToTarget" true)
          (`/Game/Blueprints/UI/TargetUI.UpdateTargetUI` (`/Game/Blueprints/UI/HeadsUpDisplay.TargetUI` (`self.Heads Up Display`))))))))

(fn `UpdateCosts`
  (bind (_ability_details_name _ability_details_description _ability_details_levelreq _ability_details_manacost _ability_details_staminacost _ability_details_cooldown _ability_details_casttime _ability_details_basepower _ability_details_isinterruptible _ability_details_icon _ability_details_tags _ability_details_validtargetlist _ability_details_healingspell_ _ability_details_range) (break `/Game/Blueprints/Abilities/AbilityDetails` (`self.Ability Details`)))
  (bind _playerref (`self.PlayerRef`))
  (set `self.Default ManaCost` _ability_details_manacost)
  (for _array_element (`/Game/Blueprints/Vocations/Vocation_Parent.UnlockedTraitList` (`/Game/Blueprints/Player/ThirdPersonCharacter.CurrentVocation` _playerref))
    (cast `/Game/Blueprints/Vocations/Vocation_Traits/Holy_Aura/Trait_HolyAura_I` _array_element
      (:`then`
        _)
      (:`CastFailed`
        (cast `/Game/Blueprints/Vocations/Vocation_Traits/Holy_Aura/Trait_HolyAura_II` _array_element
          (:`then`
            _)
          (:`CastFailed`
            (cast `/Game/Blueprints/Vocations/Vocation_Traits/Holy_Aura/Trait_HolyAura_III` _array_element)))))
    (if _ability_details_healingspell_
      (set `self.Ability Details` (make `/Game/Blueprints/Abilities/AbilityDetails` _ability_details_name _ability_details_description _ability_details_levelreq (* (`self.Default ManaCost`) (`/Game/Blueprints/Player/ThirdPersonCharacter.ManaCostMultiplier` _playerref)) _ability_details_staminacost _ability_details_cooldown _ability_details_casttime _ability_details_basepower _ability_details_isinterruptible _ability_details_icon _ability_details_tags _ability_details_validtargetlist _ability_details_healingspell_ _ability_details_range)))))

(fn `UserConstructionScript`)