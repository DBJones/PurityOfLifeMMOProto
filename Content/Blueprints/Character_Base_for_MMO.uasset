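; Base character Blueprint for an MMO, providing stat calculations and combat UI helpers.
; Supporting stats are copied from the current weapon's details, or mostly zeroed without one.
; HP regen combines trait-scaled base regen with Resolve and a combat multiplier, while the level multiplier is the square root of display level.
; Helpers bind the nameplate widget to the character and add damage-number widgets, named by the causing ability, to a container.
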(fn `CalculateHPRegen`
  (returns (`Out Regen` :type "Float (double-precision)"))
  (if (`self.InCombat?`)
    (bind _output_get (set `self.Current HP Regen` (+ (* (`self.Combat Regen Multiplier`) (`self.HP Regen Trait Multiplier`) (`self.Base HP Regen`)) (/ (`self.TotalResolve`) 4.0))))
    (return _output_get)
    (else
      (bind _output_get_2 (set `self.Current HP Regen` (+ (* (`self.HP Regen Trait Multiplier`) (`self.Base HP Regen`)) (/ (`self.TotalResolve`) 4.0))))
      (return _output_get_2))))

(fn `CalculateLevelMult`
  (returns (OutInfo :type "Float (double-precision)"))
  (return (`KismetMathLibrary.Sqrt` (`KismetMathLibrary.Conv_IntToDouble` (`self.DisplayLevel`)))))

(fn `CalculateSupportingStats`
  (bind _currentweapon (`self.CurrentWeapon`))
  (bind _weapondetails (`/Game/Blueprints/Items/Weapons/Weapon_Parent.WeaponDetails` _currentweapon))
  (`/Engine/EditorBlueprintResources/StandardMacros.IsValid` _currentweapon
    (:`Is Valid`
      (set `self.TotalWeaponStrength` (`KismetMathLibrary.FTrunc` (`.WeaponStrength_5_971B148F408D0CCB4F0CB3971DA86206` (break `/Game/Blueprints/Items/Weapons/WeaponDetails` _weapondetails))))
      (set `self.TotalWillpower` (`.Willpower_16_864AC3944E4D37979FF7D6B16595DAE2` (break `/Game/Blueprints/Items/Weapons/AugmentationCrystalStats` (`.BonusStats_78_CEE3F41141153214D74204BA7F21A501` (break `/Game/Blueprints/Items/Weapons/WeaponDetails` _weapondetails)))))
      (set `self.InnerGlow` (`.InnerGlow_23_26104B8147B1D16CA4B5C5B81836EC36` (break `/Game/Blueprints/Items/Weapons/AugmentationCrystalStats` (`.BonusStats_78_CEE3F41141153214D74204BA7F21A501` (break `/Game/Blueprints/Items/Weapons/WeaponDetails` _weapondetails)))))
      (set `self.TotalIntelligence` (`.Intelligence_22_BE27CCE84B8A93A583843791C034686C` (break `/Game/Blueprints/Items/Weapons/AugmentationCrystalStats` (`.BonusStats_78_CEE3F41141153214D74204BA7F21A501` (break `/Game/Blueprints/Items/Weapons/WeaponDetails` _weapondetails)))))
      (set `self.Total Resillience` (`.Resillience_27_534CBF104C0EEB69B5AD2E80E846E1BA` (break `/Game/Blueprints/Items/Weapons/AugmentationCrystalStats` (`.BonusStats_78_CEE3F41141153214D74204BA7F21A501` (break `/Game/Blueprints/Items/Weapons/WeaponDetails` _weapondetails)))))
      (set `self.Prestige` (`.Prestige_33_D73EAEE149DB4D8F09C3098A3FC9183D` (break `/Game/Blueprints/Items/Weapons/WeaponDetails` _weapondetails)))
      (set `self.Endurance` (`.Endurance_32_FC9AE93A4583EA6F3A1FFFA30C616BB2` (break `/Game/Blueprints/Items/Weapons/WeaponDetails` _weapondetails)))
      (set `self.TotalVitality` (`.Vitality_31_5912543447AF3329D5C28AAB2E73089B` (break `/Game/Blueprints/Items/Weapons/WeaponDetails` _weapondetails)))
      (set `self.Total Dexterity` (`KismetMathLibrary.Conv_IntToDouble` (`.Dexterity_17_F1A312084853694128C3149791A9EA8E` (break `/Game/Blueprints/Items/Weapons/AugmentationCrystalStats` (`.BonusStats_78_CEE3F41141153214D74204BA7F21A501` (break `/Game/Blueprints/Items/Weapons/WeaponDetails` _weapondetails))))))
      (set `self.Total  Vigor` (`KismetMathLibrary.Conv_IntToDouble` (`.Vigor_15_3D73985A424B714A1DCE28835325B7F4` (break `/Game/Blueprints/Items/Weapons/AugmentationCrystalStats` (`.BonusStats_78_CEE3F41141153214D74204BA7F21A501` (break `/Game/Blueprints/Items/Weapons/WeaponDetails` _weapondetails))))))
      (set `self.Total Plasticity` (`KismetMathLibrary.Conv_IntToDouble` (`.Plasticity_24_C7C730354FB2D461BFFF08A1298EE51B` (break `/Game/Blueprints/Items/Weapons/AugmentationCrystalStats` (`.BonusStats_78_CEE3F41141153214D74204BA7F21A501` (break `/Game/Blueprints/Items/Weapons/WeaponDetails` _weapondetails))))))
      (set `self.TotalResolve` (`KismetMathLibrary.Conv_IntToDouble` (break `/Game/Blueprints/Items/Weapons/AugmentationCrystalStats` (`.BonusStats_78_CEE3F41141153214D74204BA7F21A501` (break `/Game/Blueprints/Items/Weapons/WeaponDetails` _weapondetails))))))
    (:`Is Not Valid`
      (set `self.TotalWillpower` 0)
      (set `self.TotalWillpower` 0)
      (set `self.TotalIntelligence` 0)
      (set `self.TotalIntelligence` 0)
      (set `self.Total Resillience` 0)
      (set `self.Prestige` 0)
      (set `self.Endurance` 0)
      (set `self.TotalVitality` 0)
      (set `self.Total Dexterity` 0.0)
      (set `self.Total  Vigor` 0.0)
      (set `self.Total Plasticity` 0.0)
      (set `self.TotalResolve` 0.0))))

(fn `CreateNamePlate`
  (bind _asname_plate (cast `/Game/Blueprints/UI/CharacterUI/NamePlate` (`WidgetComponent.GetWidget` (`self.NamePlate`))))
  (set `/Game/Blueprints/UI/CharacterUI/NamePlate.Owner` self _asname_plate))

(fn `UpdateDamageUI`
  (params (DamageAmount :type "Float (double-precision)") (DamageCauser :type "/Game/Blueprints/Abilities/Ability Object Reference"))
  (returns (WidgetRef :type "/Game/Blueprints/UI/CharacterUI/DamageNumber Object Reference"))
  (bind _ability_details_name (break `/Game/Blueprints/Abilities/AbilityDetails` (`/Game/Blueprints/Abilities/Ability.Ability Details` DamageCauser)))
  (bind _asdamage_number_container (cast `/Game/Blueprints/UI/CharacterUI/DamageNumber_Container` (`WidgetComponent.GetWidget` (`self.DamageNum`))))
  (bind _returnvalue (`|CreateWidget` "/Game/Blueprints/UI/CharacterUI/DamageNumber.DamageNumber_C" null _ability_details_name DamageAmount))
  (`StackBox.AddChildToStackBox` (`/Game/Blueprints/UI/CharacterUI/DamageNumber_Container.UIContainer` _asdamage_number_container) _returnvalue)
  (return _returnvalue))

(fn `UserConstructionScript`)