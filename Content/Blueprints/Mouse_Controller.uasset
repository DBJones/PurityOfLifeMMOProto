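; Player controller for mouse-driven play that handles player spawning, HUD input and targeting.
; On BeginPlay, the local controller calls ServerSpawnPlayer, which delegates spawning to the PC_Mouse_Controls game mode, then creates the HUD and enables the cursor with Game and UI input.
; Input actions forward spellbook, inventory and quest log requests to the HUD widget.
; SetTarget stores the player's target and fires the TargetChanged dispatcher.
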(event `ServerSpawnPlayer`
  (bind _aspc_mouse_controls (cast `/Game/Blueprints/PC_Mouse_Controls` (`GameplayStatics.GetGameMode`)))
  (`/Game/Blueprints/PC_Mouse_Controls.SpawnPlayer` _aspc_mouse_controls self))

(event `GenerateCharacters`)

(event `self.ReceiveBeginPlay`
  (if (`self.IsLocalPlayerController`)
    (`self.ServerSpawnPlayer`)
    (bind _returnvalue (`|CreateWidget` "/Game/Blueprints/UI/CharacterUI/HeadsUpDisplay.HeadsUpDisplay_C" null null))
    (set `self.W_HUD` _returnvalue)
    (`UserWidget.AddToViewport` _returnvalue 0)
    (`WidgetBlueprintLibrary.SetInputMode_GameAndUIEx` self null "DoNotLock" false)
    (set `self.bShowMouseCursor` true)))

(event `InputAction|OpenSpellbook`
  (params (Key :type "Key Structure"))
  (:`Pressed`
    (`/Game/Blueprints/UI/CharacterUI/HeadsUpDisplay.ToggleSpellbook` (`self.W_HUD`))))

(event `InputAction|DisplayInventory`
  (params (Key :type "Key Structure"))
  (:`Pressed`
    (`/Game/Blueprints/UI/CharacterUI/HeadsUpDisplay.DisplayPlayerInventory` (`self.W_HUD`))))

(event `InputAction|OpenQuestLog`
  (params (Key :type "Key Structure"))
  (:`Pressed`
    (`/Game/Blueprints/UI/CharacterUI/HeadsUpDisplay.OpenQuestLog` (`self.W_HUD`))))

(fn `SetTarget`
  (params (Target :type "/Game/Blueprints/Character_Base_for_MMO Object Reference"))
  (set `self.PlayerTarget` Target)
  (`self.TargetChanged`))

(fn `UserConstructionScript`)